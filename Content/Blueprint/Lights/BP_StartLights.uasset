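; BP_StartLights is a trigger that starts a set of crystal lights the first time the player character overlaps its box.
; The overlap event passes through a DoOnce and hands the CrystalLights array to its SetIntensity function.
; That function loops over the crystals, calling each one's SetIntensity with a Delay value that grows by one per element, which suggests a staggered sequence.
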(event `self.Box.OnComponentBeginOverlap`
  (params (OverlappedComponent :type "PrimitiveComponent Object Reference") (OtherActor :type "Actor Object Reference") (OtherComp :type "PrimitiveComponent Object Reference") (OtherBodyIndex :type Integer) (bFromSweep :type Boolean) (SweepResult :type "HitResult Structure (by ref)"))
  (if (== OtherActor (`GameplayStatics.GetPlayerCharacter` 0))
    (`/Engine/EditorBlueprintResources/StandardMacros.DoOnce` false
      (:`Completed`
        (`self.SetIntensity` (`self.CrystalLights`))))))

(fn `SetIntensity`
  (params (Crystals :type "Array of /Game/Blueprint/Lights/BP_CrystalLights Object Reference"))
  (locals (Delay :type "Float (double-precision)"))
  (for _array_element Crystals
    (bind _output_get (set `local.Delay` (+ (`local.Delay`) 1.0)))
    (`/Game/Blueprint/Lights/BP_CrystalLights.SetIntensity` _array_element _output_get)))

(fn `UserConstructionScript`)