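; BP_CrystalLights is a crystal light that starts with its glow off and fades on when triggered.
; The construction script applies the chosen material and light colour, and BeginPlay creates a dynamic material instance with Emissive at zero.
; SetIntensity waits a given delay, then a timeline ramps the point light's intensity and the crystal's Emissive parameter up together.
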(event `self.ReceiveBeginPlay`
  (bind _returnvalue (`PrimitiveComponent.CreateDynamicMaterialInstance` (`self.CrystalTemp`) 0 (`self.Material`) "None"))
  (`MaterialInstanceDynamic.SetScalarParameterValue` _returnvalue "Emissive" 0.0)
  (set `self.DM_Cry` _returnvalue))

(event `SetIntensity`
  (params (Delay :type "Float (double-precision)"))
  (`KismetSystemLibrary.Delay` Delay)
  (bind (_direction _alpha) (`Timeline|LightIntensityTL`)
    (:`Update`
      (`LightComponent.SetIntensity` (`self.PointLight`) (`KismetMathLibrary.Lerp` 0.0 (`self.Intensity`) _alpha))
      (`MaterialInstanceDynamic.SetScalarParameterValue` (`self.DM_Cry`) "Emissive" (`KismetMathLibrary.Lerp` 0.0 1.0 _alpha)))))

(fn `UserConstructionScript`
  (`PrimitiveComponent.SetMaterial` (`self.CrystalTemp`) 0 (`self.Material`))
  (`LightComponent.SetLightColor` (`self.PointLight`) (`self.LightColour`) true))