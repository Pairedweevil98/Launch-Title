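; BP_SwingLights is a trigger that sets a group of lights swinging when the player walks into it.
; When its Box overlaps the player character, it loops over the Lights array and calls Swing on each entry.
; Each light gets its own random X and Y swing amounts between SwingAmountMin and SwingAmountMax, with no swing on Z.
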(event `self.Box.OnComponentBeginOverlap`
  (params (OverlappedComponent :type "PrimitiveComponent Object Reference") (OtherActor :type "Actor Object Reference") (OtherComp :type "PrimitiveComponent Object Reference") (OtherBodyIndex :type Integer) (bFromSweep :type Boolean) (SweepResult :type "HitResult Structure (by ref)"))
  (if (== OtherActor (`GameplayStatics.GetPlayerCharacter` 0))
    (for _array_element (`self.Lights`)
      (`/Game/Blueprint/Lights/BP_SwingingLight.Swing` _array_element (`KismetMathLibrary.MakeVector` (`KismetMathLibrary.RandomFloatInRange` (`self.Swing AmountMin`) (`self.SwingAmountMax`)) (`KismetMathLibrary.RandomFloatInRange` (`self.Swing AmountMin`) (`self.SwingAmountMax`)))))))

(fn `UserConstructionScript`)