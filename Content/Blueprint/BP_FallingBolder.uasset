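; BP_FallingBolder is a boulder hazard that can kill the player character in a side-scroller.
; Only the first player hit is evaluated through a DoOnce, calling Death on the SideScrollerCharacter if the boulder's Y velocity exceeds a small threshold.
; Hits on anything else play a world camera shake at the boulder.
; A separate CameraShake event, not called here, plays another shake over a wider radius.
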(event `self.Bolder.OnComponentHit`
  (params (HitComponent :type "PrimitiveComponent Object Reference") (OtherActor :type "Actor Object Reference") (OtherComp :type "PrimitiveComponent Object Reference") (NormalImpulse :type "Vector Structure") (Hit :type "HitResult Structure (by ref)"))
  (bind (_returnvalue_x _returnvalue_y) (`KismetMathLibrary.BreakVector` (`SceneComponent.GetComponentVelocity` (`self.Bolder`))))
  (if (== OtherActor (`GameplayStatics.GetPlayerCharacter` 0))
    (`/Engine/EditorBlueprintResources/StandardMacros.DoOnce` false
      (:`Completed`
        (if (> _returnvalue_y 5.0)
          (bind _asside_scroller_character (cast `/Game/SideScrollerBP/Blueprints/SideScrollerCharacter` OtherActor))
          (`/Game/SideScrollerBP/Blueprints/SideScrollerCharacter.Death` _asside_scroller_character))))
    (else
      (`GameplayStatics.PlayWorldCameraShake` "/Game/Blueprint/Camera/BolderCamShake1.BolderCamShake1_C" (`self.K2_GetActorLocation`) 0.0 5000.0))))

(event `CameraShake`
  (`GameplayStatics.PlayWorldCameraShake` "/Game/Blueprint/Camera/BolderCamShake.BolderCamShake_C" (`self.K2_GetActorLocation`) 0.0 25000.0))

(fn `UserConstructionScript`)