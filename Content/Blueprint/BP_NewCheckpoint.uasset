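; BP_NewCheckpoint is a side-scroller torch checkpoint that lights up the first time the SideScrollerCharacter enters its Box.
; The overlap saves the Box location as LastCheckpoint, with X fixed to a constant.
; The SetLight timeline ramps the point light and a dynamic material's Emission, starting the fire sound and toggling the fireflies Niagara effect once.
; When it finishes, FlickerTL takes over the light intensity for flickering.
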(event `self.ReceiveBeginPlay`
  (bind _returnvalue (`PrimitiveComponent.CreateDynamicMaterialInstance` (`self.Cube`) 0 "/Game/Materials/MI_EmisTourch.MI_EmisTourch" "None"))
  (`AudioComponent.Stop` (`self.FireSound`)))

(event `self.Box.OnComponentBeginOverlap`
  (params (OverlappedComponent :type "PrimitiveComponent Object Reference") (OtherActor :type "Actor Object Reference") (OtherComp :type "PrimitiveComponent Object Reference") (OtherBodyIndex :type Integer) (bFromSweep :type Boolean) (SweepResult :type "HitResult Structure (by ref)"))
  (bind (_returnvalue_x _returnvalue_y _returnvalue_z) (`KismetMathLibrary.BreakVector` (`SceneComponent.K2_GetComponentLocation` (`self.Box`))))
  (bind _asside_scroller_character (cast `/Game/SideScrollerBP/Blueprints/SideScrollerCharacter` OtherActor))
  (`/Engine/EditorBlueprintResources/StandardMacros.DoOnce` false
    (:`Completed`
      (set `/Game/SideScrollerBP/Blueprints/SideScrollerCharacter.LastCheckpoint` (`KismetMathLibrary.MakeVector` 1200.0 _returnvalue_y _returnvalue_z) _asside_scroller_character)
      (bind (_direction _lightintensity) (`Timeline|SetLight`)
        (:`Update`
          (`LightComponent.SetIntensity` (`self.PointLight`) (`KismetMathLibrary.Lerp` 0.0 2500.0 _lightintensity))
          (`MaterialInstanceDynamic.SetScalarParameterValue` (stale `self.ReceiveBeginPlay` _returnvalue) "Emission" (`KismetMathLibrary.Lerp` 0.0 20.0 _lightintensity))
          (`/Engine/EditorBlueprintResources/StandardMacros.DoOnce` false
            (:`Completed`
              (`AudioComponent.Play` (`self.FireSound`) 0.0)
              (`ActorComponent.ToggleActive` (`self.NS_FireFliesTourch`)))))
        (:`Finished`
          (bind (_direction_2 _lightintensity_2) (`Timeline|FlickerTL`)
            (:`Update`
              (`LightComponent.SetIntensity` (`self.PointLight`) (`KismetMathLibrary.Lerp` 0.0 2500.0 _lightintensity_2)))))))))

(fn `UserConstructionScript`)