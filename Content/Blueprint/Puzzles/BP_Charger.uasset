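; Puzzle charger that a light beam powers once to open a linked door or power a linked lever.
; On light interaction it waits briefly, confirms the beam still hits it, then plays a one-time timeline.
; The timeline ramps emission on dynamic materials for its cube and crystal chunk.
; When the glow finishes, it calls OpenDoor on any valid Door and SetPowered on any valid Lever.
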(event `self.ReceiveBeginPlay`
  (bind _returnvalue (`PrimitiveComponent.CreateDynamicMaterialInstance` (`self.Cube`) 0 "/Game/Materials/MI_LightBeam.MI_LightBeam" "None"))
  (bind _returnvalue_2 (`PrimitiveComponent.CreateDynamicMaterialInstance` (`self.Crystal_Chunk`) 0 null "None")))

(event `/Game/Blueprint/BPI_LightBeamInteract.OnLightInteract`
  (params (LightBeam :type "/Game/Blueprint/Puzzles/BP_laser Object Reference"))
  (`KismetSystemLibrary.Delay` 1.0)
  (if (== (`/Game/Blueprint/Puzzles/BP_laser.HitActor` LightBeam) self)
    (`/Engine/EditorBlueprintResources/StandardMacros.DoOnce` false
      (:`Completed`
        (bind (_direction _emission) (`Timeline|Emission`)
          (:`Update`
            (`MaterialInstanceDynamic.SetScalarParameterValue` (stale `self.ReceiveBeginPlay` _returnvalue) "Emission" (`KismetMathLibrary.Lerp` 1.0 35.0 _emission))
            (`MaterialInstanceDynamic.SetScalarParameterValue` (stale `self.ReceiveBeginPlay` _returnvalue_2) "Emission" (`KismetMathLibrary.Lerp` 1.0 35.0 _emission)))
          (:`Finished`
            (`self.CallDoor`)))))))

(event `CallDoor`
  (bind _door (`self.Door`))
  (bind _lever (`self.Lever`))
  (`/Engine/EditorBlueprintResources/StandardMacros.IsValid` _door
    (:`Is Valid`
      (`/Game/Blueprint/Puzzles/BP_Door.OpenDoor` _door))
    (:`Is Not Valid`
      _))
  (`/Engine/EditorBlueprintResources/StandardMacros.IsValid` _lever
    (:`Is Valid`
      (bind _output_get (set `/Game/Blueprint/Platforms/BP_Lever.Powered` true _lever))
      (`/Game/Blueprint/Platforms/BP_Lever.SetPowered` _lever _output_get))))

(fn `UserConstructionScript`)