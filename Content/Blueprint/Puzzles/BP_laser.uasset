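; Puzzle laser emitter that switches on at first interaction, then rotates in timeline-driven turns, reversing timelines after a set number of turns.
; A repeating update traces from the arrow, mirroring the ray off surfaces using MI_LightBeam and rebuilding BP_LaserBeam actors for each segment.
; The final hit receives damage and interact messages if it implements either interface.
; Lighting up also ramps the crystal's emission through a dynamic material.
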(event `/Game/Blueprint/BPI_Interact.Interact`
  (params (Player :type "/Game/SideScrollerBP/Blueprints/SideScrollerCharacter Object Reference"))
  (bind _staticmesh (`self.StaticMesh`))
  (if (`self.LightOn?`)
    (if (`self.AddOrSub`)
      (`/Engine/EditorBlueprintResources/StandardMacros.DoOnce` false :!label _label
        (:`Completed`
          (bind (_direction _rotatetrack) (`Timeline|Timeline_0` :!via `PlayFromStart`)
            (:`Update`
              (bind _returnvalue (+ _rotatetrack (`self.CurrentRotation`)))
              (`SceneComponent.K2_SetWorldRotation` _staticmesh (`KismetMathLibrary.MakeRotator` _returnvalue) false false)
              (`self.CastLight`))
            (:`Finished`
              (set `self.CurrentRotation` _returnvalue)
              (`|ExecutionSequence`
                (:`then_0`
                  (bind _result (`/Engine/EditorBlueprintResources/StandardMacros.IncrementInt` (`self.CurrentTurn`))
                    (:`  `
                      (if (> _result 3)
                        (set `self.AddOrSub` false)
                        (set `self.CurrentTurn` 0)))))
                (:`then_1`
                  (goto _label :!via `Reset`)))))))
      (else
        (`/Engine/EditorBlueprintResources/StandardMacros.DoOnce` false :!label _label_2
          (:`Completed`
            (bind (_direction_2 _rotatetrack_2) (`Timeline|Timeline_1` :!via `PlayFromStart`)
              (:`Update`
                (bind _returnvalue_2 (+ _rotatetrack_2 (`self.CurrentRotation`)))
                (`SceneComponent.K2_SetWorldRotation` _staticmesh (`KismetMathLibrary.MakeRotator` _returnvalue_2) false false)
                (`self.CastLight`))
              (:`Finished`
                (set `self.CurrentRotation` _returnvalue_2)
                (`|ExecutionSequence`
                  (:`then_0`
                    (bind _result_2 (`/Engine/EditorBlueprintResources/StandardMacros.IncrementInt` (`self.CurrentTurn`))
                      (:`  `
                        (if (> _result_2 3)
                          (set `self.AddOrSub` true)
                          (set `self.CurrentTurn` 0)))))
                  (:`then_1`
                    (goto _label_2 :!via `Reset`)))))))))
    (else
      (`self.CastLight`))))

(event `CastLight`
  (bind _arrow (`self.Arrow`))
  (set `self.LightOn?` true)
  (`Timeline|RepeatLightBeam`
    (:`Update`
      (`self.LightRay` (`SceneComponent.K2_GetComponentLocation` _arrow) (`SceneComponent.GetForwardVector` _arrow) (`self.Distance`))
      (`/Engine/EditorBlueprintResources/StandardMacros.DoOnce` false
        (:`Completed`
          (bind (_direction _emission) (`Timeline|SetEmission`)
            (:`Update`
              (`MaterialInstanceDynamic.SetScalarParameterValue` (stale `self.ReceiveBeginPlay` _returnvalue) "Emission" (`KismetMathLibrary.Lerp` 1.0 35.0 _emission)))))))))

(event `self.ReceiveBeginPlay`
  (bind _returnvalue (`PrimitiveComponent.CreateDynamicMaterialInstance` (`self.Crystal`) 0 "/Game/Materials/MI_LightBeam.MI_LightBeam" "None")))

(fn `LightRay`
  (params (OriginLoc :type "Vector Structure") (Direction :type "Vector Structure") (Distance :type "Float (double-precision)"))
  (locals (L_OriginLoc :type "Vector Structure") (L_Direction :type "Vector Structure") (L_Distance :type "Float (double-precision)") (L_Continue :type Boolean :default true) (L_StartBeamLoc :type "Vector Structure") (L_EndBeamLoc :type "Vector Structure"))
  (bind _l_originloc (`local.L_OriginLoc`))
  (bind _beams (`self.Beams`))
  (set `local.L_OriginLoc` OriginLoc)
  (set `local.L_Direction` Direction)
  (set `local.L_Distance` Distance)
  (for _array_element _beams
    (`self.K2_DestroyActor` _array_element))
  (`KismetArrayLibrary.Array_Clear` _beams)
  (while (`local.L_Continue`)
    (`|ExecutionSequence`
      (:`then_0`
        (bind (_outhit _returnvalue) (`KismetSystemLibrary.LineTraceSingle` _l_originloc (+ _l_originloc (* (`local.L_Direction`) (`local.L_Distance`))) "TraceTypeQuery3" true))
        (set `local.L_StartBeamLoc` (`local.L_OriginLoc`))
        (if _returnvalue
          (bind (_bblockinghit _binitialoverlap _time _distance _location _impactpoint _normal _impactnormal _physmat _hitactor _hitcomponent _hitbonename _hititem _faceindex _tracestart _traceend) (`GameplayStatics.BreakHitResult` _outhit))
          (set `local.L_EndBeamLoc` _impactpoint)
          (if (== (`.ReturnValue` (`PrimitiveComponent.GetMaterialFromCollisionFaceIndex` _hitcomponent _faceindex)) "/Game/Materials/MI_LightBeam.MI_LightBeam")
            (set `local.L_OriginLoc` _impactpoint)
            (set `local.L_Direction` (`KismetMathLibrary.MirrorVectorByNormal` (`local.L_Direction`) _impactnormal))
            (set `local.L_Continue` true)
            (else
              (if (or (`KismetSystemLibrary.DoesImplementInterface` _hitactor "/Game/Blueprint/BPI_Interact.BPI_Interact_C") (`KismetSystemLibrary.DoesImplementInterface` _hitactor "/Game/Blueprint/BPI_Damage.BPI_Damage_C"))
                (message `/Game/Blueprint/BPI_Damage.TakeDamage` _hitactor)
                (message `/Game/Blueprint/BPI_Interact.Interact` _hitactor null))
              (set `local.L_Continue` false :!label _label)))
          (else
            (set `local.L_EndBeamLoc` _traceend)
            (goto _label))))
      (:`then_1`
        (bind _returnvalue_2 (`|SpawnActorFromClass` "/Game/Blueprint/Puzzles/BP_LaserBeam.BP_LaserBeam_C" (`KismetMathLibrary.MakeTransform` (0.0 0.0 0.0)) "Undefined" "OverrideRootScale" null null))
        (`/Game/Blueprint/Puzzles/BP_LaserBeam.Set End` _returnvalue_2 (`local.L_StartBeamLoc`) (`local.L_EndBeamLoc`))
        (`KismetArrayLibrary.Array_Add` (`self.Beams`) _returnvalue_2)))))

(fn `UserConstructionScript`)