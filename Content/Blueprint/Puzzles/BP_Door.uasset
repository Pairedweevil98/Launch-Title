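; Puzzle door that slides its Cube along local X when OpenDoor or CloseDoor is called.
; The OpenClose timeline drives the slide, playing forward once to open and reversing to close, with a world camera shake either way.
; If IsCollisionBox is set, a SideScrollerCharacter entering the Box while pushing an object closes the door once.
; The construction script positions that trigger from BoxTransform.
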(event `OpenDoor`
  (`/Engine/EditorBlueprintResources/StandardMacros.DoOnce` false
    (:`Completed`
      (`|ExecutionSequence`
        (:`then_0`
          (bind (_direction _openorclose) (`Timeline|OpenClose` :!via `PlayFromStart` :!label _label)
            (:`Update`
              (`SceneComponent.K2_SetRelativeLocation` (`self.Cube`) (`KismetMathLibrary.MakeVector` (`KismetMathLibrary.Lerp` 0.0 -380.0 _openorclose)) false false))))
        (:`then_1`
          (`GameplayStatics.PlayWorldCameraShake` "/Game/Blueprint/Camera/DoorOpeningCamShake.DoorOpeningCamShake_C" (`self.K2_GetActorLocation`) 0.0 5000.0 1.0 true :!label _label_2))))))

(event `CloseDoor`
  (`|ExecutionSequence`
    (:`then_0`
      (goto _label :!via `Reverse`))
    (:`then_1`
      (goto _label_2))))

(event `self.Box.OnComponentBeginOverlap`
  (params (OverlappedComponent :type "PrimitiveComponent Object Reference") (OtherActor :type "Actor Object Reference") (OtherComp :type "PrimitiveComponent Object Reference") (OtherBodyIndex :type Integer) (bFromSweep :type Boolean) (SweepResult :type "HitResult Structure (by ref)"))
  (if (`self.IsCollisionBox?`)
    (bind _asside_scroller_character (cast `/Game/SideScrollerBP/Blueprints/SideScrollerCharacter` OtherActor))
    (if (`/Game/Blueprint/PushComponent.IsPushingObject` (`/Game/SideScrollerBP/Blueprints/SideScrollerCharacter.PushComponent` _asside_scroller_character))
      (`/Engine/EditorBlueprintResources/StandardMacros.DoOnce` false
        (:`Completed`
          (`self.CloseDoor`))))))

(fn `UserConstructionScript`
  (`SceneComponent.K2_SetRelativeTransform` (`self.Box`) (`self.BoxTransform`) false false))