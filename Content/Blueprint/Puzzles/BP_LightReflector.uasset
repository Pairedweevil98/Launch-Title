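; Puzzle light reflector that rotates its mirror mesh a step each time it is interacted with.
; Interact plays a timeline that adds its track value to the stored roll of StaticMesh1, then saves the new angle.
; A DoOnce blocks further interaction until the turn finishes.
; Disconnected leftover nodes for checking light sources, casting light and setting beam emission never run.
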(event `self.ReceiveBeginPlay`)

(event `/Game/Blueprint/BPI_Interact.Interact`
  (params (Player :type "/Game/SideScrollerBP/Blueprints/SideScrollerCharacter Object Reference"))
  (`/Engine/EditorBlueprintResources/StandardMacros.DoOnce` false :!label _label
    (:`Completed`
      (bind (_direction _rotatetrack) (`Timeline|RotateTimeline` :!via `PlayFromStart`)
        (:`Update`
          (bind _returnvalue (+ _rotatetrack (`self.CurrentRotation`)))
          (`SceneComponent.K2_SetRelativeRotation` (`self.StaticMesh1`) (`KismetMathLibrary.MakeRotator` _returnvalue) false false))
        (:`Finished`
          (set `self.CurrentRotation` _returnvalue)
          (goto _label :!via `Reset`))))))

(fn `UserConstructionScript`)