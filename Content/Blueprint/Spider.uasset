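; Spider hazard actor for a side-scroller that kills the player character on contact and can flee out of play.
; A Box overlap casts the other actor to SideScrollerCharacter and calls its Death function.
; The RunAway event plays the Run timeline, which moves the root along negative Y, then destroys the actor.
; Each update lerps from the current location rather than a stored start, so the movement accumulates over the timeline.
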(event `RunAway`
  (bind (_returnvalue_x _returnvalue_y _returnvalue_z) (`KismetMathLibrary.BreakVector` (`SceneComponent.K2_GetComponentLocation` (`self.DefaultSceneRoot`))))
  (bind (_direction _runtrack) (`Timeline|Run`)
    (:`Update`
      (`SceneComponent.K2_SetWorldLocation` (`self.DefaultSceneRoot`) (`KismetMathLibrary.MakeVector` _returnvalue_x (`KismetMathLibrary.Lerp` _returnvalue_y (+ _returnvalue_y -100.0) _runtrack) _returnvalue_z) false false))
    (:`Finished`
      (`self.K2_DestroyActor`))))

(event `self.Box.OnComponentBeginOverlap`
  (params (OverlappedComponent :type "PrimitiveComponent Object Reference") (OtherActor :type "Actor Object Reference") (OtherComp :type "PrimitiveComponent Object Reference") (OtherBodyIndex :type Integer) (bFromSweep :type Boolean) (SweepResult :type "HitResult Structure (by ref)"))
  (bind _asside_scroller_character (cast `/Game/SideScrollerBP/Blueprints/SideScrollerCharacter` OtherActor))
  (`/Game/SideScrollerBP/Blueprints/SideScrollerCharacter.Death` _asside_scroller_character))

(fn `UserConstructionScript`)