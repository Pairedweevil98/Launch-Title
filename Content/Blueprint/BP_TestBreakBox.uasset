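; BP_TestBreakBox is a breakable test box actor that takes damage and bursts into a coloured particle effect when destroyed.
; It applies its Colour material to the cube on BeginPlay and subtracts incoming damage from Health.
; At zero health it spawns a yellow, red or purple pickaxe-hit Niagara system chosen by ParticleColour, hides the cube, disables collision and destroys itself after a short delay.
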(event `self.ReceiveBeginPlay`
  (`PrimitiveComponent.SetMaterial` (`self.Cube`) 0 (`self.Colour`)))

(event `/Game/Blueprint/BPI_Damage.TakeDamage`
  (params (DamageAmount :type Integer))
  (bind _cube (`self.Cube`))
  (bind _output_get (set `self.Health` (- (`self.Health`) DamageAmount)))
  (if (<= _output_get 0)
    (`self.SpawnParticle` (`self.Particle Colour`))
    (`SceneComponent.SetVisibility` _cube false false)
    (`PrimitiveComponent.SetCollisionEnabled` _cube "NoCollision")
    (`KismetSystemLibrary.Delay` 2.0)
    (`self.K2_DestroyActor`)))

(fn `SpawnParticle`
  (params (ParticleColour :type "/Game/ParticleColours Enum" :default "NewEnumerator0"))
  (bind _returnvalue (`SceneComponent.K2_GetComponentLocation` (`self.Cube`)))
  (switch `/Game/ParticleColours` ParticleColour
    (:`NewEnumerator0`
      (`NiagaraFunctionLibrary.SpawnSystemAtLocation` "/Game/ParticleEffects/PickAxeSwings/NS_PickAxeHitYellow.NS_PickAxeHitYellow" _returnvalue))
    (:`NewEnumerator1`
      (`NiagaraFunctionLibrary.SpawnSystemAtLocation` "/Game/ParticleEffects/PickAxeSwings/NS_PickAxeHitRed.NS_PickAxeHitRed" _returnvalue))
    (:`NewEnumerator2`
      (`NiagaraFunctionLibrary.SpawnSystemAtLocation` "/Game/ParticleEffects/PickAxeSwings/NS_PickAxeHitPurple.NS_PickAxeHitPurple" _returnvalue)))
  (return))

(fn `UserConstructionScript`)