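; Foot IK function library that computes pelvis/root drop and per-foot offsets and rotations to fit a character's feet to uneven ground.
; FootIK traces down from capsule height at both ankle sockets; if either hits, the larger distance drives the interpolated root displacement.
; Pelvis-height traces at each ankle then give interpolated foot offsets, with uninterpolated roll and pitch derived from the surface normal.
; Callers pass in current values for smoothing.
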(fn `CalculateFootOffset`
  (params (FootDistance :type "Float (double-precision)") (CurrentFootOffset :type "Float (double-precision)") (DeltaTime :type "Float (double-precision)") (InterpSpeed :type "Float (double-precision)") (Rotation :type "Vector Structure"))
  (returns (ReturnOffset :type "Float (double-precision)") (ReturnRotation :type "Rotator Structure"))
  (return (`KismetMathLibrary.FInterpTo` CurrentFootOffset (/ (- FootDistance 110.0) -45.0) DeltaTime InterpSpeed) (`KismetMathLibrary.MakeRotator` (`KismetMathLibrary.DegAtan2` Rotation_Y Rotation_Z) (* (`KismetMathLibrary.DegAtan2` Rotation_X Rotation_Z) -1.0))))

(fn `CalculateRootDisplacement`
  (params (DistanceA :type "Float (double-precision)") (DistanceB :type "Float (double-precision)") (CurrentRootDisplacement :type "Float (double-precision)") (CapsuleHalfHeight :type "Float (double-precision)") (DeltaTime :type "Float (double-precision)") (InterpSpeed :type "Float (double-precision)"))
  (returns (ReturnValue :type "Float (double-precision)"))
  (return (`KismetMathLibrary.FInterpTo` CurrentRootDisplacement (* (- (`KismetMathLibrary.SelectFloat` DistanceA DistanceB (>= DistanceA DistanceB)) CapsuleHalfHeight) -1.0) DeltaTime InterpSpeed)))

(fn `FootIK`
  (params (Mesh :type "SceneComponent Object Reference") (InRootDisplacement :type "Float (double-precision)") (InRightFootOffset :type "Float (double-precision)") (InLeftFootOffset :type "Float (double-precision)") (CapsuleHalfHeight :type "Float (double-precision)") (DeltaTime :type "Float (double-precision)") (InterpSpeed :type "Float (double-precision)"))
  (returns (OutRootDisplacement :type "Float (double-precision)") (OutLeftFootOffset :type "Float (double-precision)") (OutRightFootOffset :type "Float (double-precision)") (OutRightFootRotation :type "Rotator Structure") (OutLeftFootRotation :type "Rotator Structure"))
  (locals (RootDisplacement :type "Float (double-precision)") (RightFootOffset :type "Float (double-precision)") (LeftFootOffset :type "Float (double-precision)") (RightFootRotation :type "Rotator Structure" :default (struct)) (LeftFootRotation :type "Rotator Structure" :default (struct)))
  (bind (_bblockinghit _distance) (`self.GetRootDisplacement` "Ankle_R" Mesh CapsuleHalfHeight))
  (bind (_bblockinghit_2 _distance_2) (`self.GetRootDisplacement` "Ankle_L" Mesh CapsuleHalfHeight))
  (if (or _bblockinghit_2 _bblockinghit)
    (bind _returnvalue (`self.CalculateRootDisplacement` _distance_2 _distance InRootDisplacement CapsuleHalfHeight DeltaTime InterpSpeed))
    (set `local.RootDisplacement` _returnvalue)
    (bind (_bblockinghit_3 _distance_3 _normal) (`self.GetFootPosition` "Ankle_R" Mesh))
    (bind (_returnoffset _returnrotation) (`self.CalculateFootOffset` _distance_3 InRightFootOffset DeltaTime InterpSpeed _normal)) ; Right
    (set `local.RightFootOffset` _returnoffset)
    (set `local.RightFootRotation` _returnrotation)
    (bind (_bblockinghit_4 _distance_4 _normal_2) (`self.GetFootPosition` "Ankle_L" Mesh))
    (bind (_returnoffset_2 _returnrotation_2) (`self.CalculateFootOffset` _distance_4 InLeftFootOffset DeltaTime InterpSpeed _normal_2)) ; Left
    (set `local.LeftFootOffset` _returnoffset_2)
    (set `local.LeftFootRotation` _returnrotation_2)
    (return (`local.RootDisplacement`) (`local.LeftFootOffset`) (`local.RightFootOffset`) (`local.RightFootRotation`) (`local.LeftFootRotation`))))

(fn `GetFootPosition`
  (params (InSocketName :type Name) (Mesh :type "SceneComponent Object Reference"))
  (returns (bBlockingHit :type Boolean) (Distance :type "Float (double-precision)") (Normal :type "Vector Structure"))
  (bind (_returnvalue_x _returnvalue_y _returnvalue_z) (`KismetMathLibrary.BreakVector` (`SceneComponent.GetSocketLocation` Mesh "Pelvis")))
  (bind (_returnvalue_x_2 _returnvalue_y_2) (`KismetMathLibrary.BreakVector` (`SceneComponent.GetSocketLocation` Mesh InSocketName)))
  (bind _returnvalue (`KismetMathLibrary.MakeVector` _returnvalue_x_2 _returnvalue_y_2 _returnvalue_z))
  (bind (_outhit _returnvalue_2) (`KismetSystemLibrary.LineTraceSingle` null (+ _returnvalue (0.0 0.0 100.0)) (- _returnvalue (0.0 0.0 100.0)) "TraceTypeQuery1"))
  (if _returnvalue_2
    (bind (_bblockinghit _binitialoverlap _time _distance _location _impactpoint _normal) (`GameplayStatics.BreakHitResult` _outhit))
    (return _bblockinghit _distance _normal)
    (else
      (return _bblockinghit 9999.0 (0.0 0.0 0.0)))))

(fn `GetRootDisplacement`
  (params (InSocketName :type Name) (Mesh :type "SceneComponent Object Reference") (CapsuleHalfHeight :type "Float (double-precision)"))
  (returns (bBlockingHit :type Boolean) (Distance :type "Float (double-precision)"))
  (bind (_returnvalue_x _returnvalue_y) (`KismetMathLibrary.BreakVector` (`SceneComponent.GetSocketLocation` Mesh InSocketName)))
  (bind (_returnvalue_x_2 _returnvalue_y_2 _returnvalue_z) (`KismetMathLibrary.BreakVector` (+ (`SceneComponent.K2_GetComponentLocation` Mesh) (`KismetMathLibrary.MakeVector` 0.0 0.0 CapsuleHalfHeight))))
  (bind _returnvalue (`KismetMathLibrary.MakeVector` _returnvalue_x _returnvalue_y _returnvalue_z))
  (bind _outhit (`KismetSystemLibrary.LineTraceSingle` null _returnvalue (- _returnvalue (0.0 0.0 151.0)) "TraceTypeQuery1"))
  (bind (_bblockinghit _binitialoverlap _time _distance) (`GameplayStatics.BreakHitResult` _outhit))
  (return _bblockinghit _distance))