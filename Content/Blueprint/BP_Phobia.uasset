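; BP_Phobia is a spider enemy that kills the SideScrollerCharacter when it overlaps its box.
; Tick checks player distance, with two DoOnce gates firing hostile or cool-down montages and sounds once per range change.
; A light beam still hitting it after a short delay starts a timeline that raises it, then destroys it.
; The construction script snaps a slime effect to the skeletal mesh's head socket.
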(event `self.ReceiveTick`
  (params (DeltaSeconds :type "Float (single-precision)"))
  (bind _returnvalue (`self.K2_GetActorLocation`))
  (bind _skeletalmesh (`self.SkeletalMesh`))
  (bind _output_get (set `self.Player Distance` (`KismetMathLibrary.VSize` (- (`self.K2_GetActorLocation`) (`self.K2_GetActorLocation` (`GameplayStatics.GetPlayerCharacter` 0))))))
  (if (< _output_get 1000.0)
    (`/Engine/EditorBlueprintResources/StandardMacros.DoOnce` false :!label _label
      (:`Completed`
        (`|ExecutionSequence`
          (:`then_0`
            (`|PlayMontage` _skeletalmesh "/Game/Teammates/Danielle/Phobia_Hostile_Montage.Phobia_Hostile_Montage"
              (:`then`
                (`GameplayStatics.PlaySoundAtLocation` "/Game/Sounds/SpiderHostile.SpiderHostile" _returnvalue (struct) 1.0 1.0 0.0 null null null))))
          (:`then_1`
            (goto _label_2 :!via `Reset`)))))
    (else
      (`|ExecutionSequence`
        (:`then_0`
          (goto _label :!via `Reset`))
        (:`then_1`
          (`/Engine/EditorBlueprintResources/StandardMacros.DoOnce` false :!label _label_2
            (:`Completed`
              (`|PlayMontage` _skeletalmesh "/Game/Teammates/Danielle/Phobia_Hostile_Cool_Down_Montage.Phobia_Hostile_Cool_Down_Montage"
                (:`then`
                  (`GameplayStatics.PlaySoundAtLocation` "/Game/Sounds/SpiderIdle.SpiderIdle" _returnvalue (struct) 1.0 1.0 0.0 null null null))))))))))

(event `/Game/Blueprint/BPI_LightBeamInteract.OnLightInteract`
  (params (LightBeam :type "/Game/Blueprint/Puzzles/BP_Projector Object Reference"))
  (bind (_returnvalue_x _returnvalue_y _returnvalue_z) (`KismetMathLibrary.BreakVector` (`SceneComponent.K2_GetComponentLocation` (`self.DefaultSceneRoot`))))
  (`KismetSystemLibrary.Delay` 1.0)
  (if (== (`/Game/Blueprint/Puzzles/BP_Projector.HitActor` LightBeam) self)
    (bind (_direction _runtrack) (`Timeline|Timeline_0`)
      (:`Update`
        (`SceneComponent.K2_SetWorldLocation` (`self.DefaultSceneRoot`) (`KismetMathLibrary.MakeVector` _returnvalue_x _returnvalue_y (`KismetMathLibrary.Lerp` _returnvalue_z (+ _returnvalue_z 100.0) _runtrack)) false false))
      (:`Finished`
        (`self.K2_DestroyActor`)))))

(event `self.Box.OnComponentBeginOverlap`
  (params (OverlappedComponent :type "PrimitiveComponent Object Reference") (OtherActor :type "Actor Object Reference") (OtherComp :type "PrimitiveComponent Object Reference") (OtherBodyIndex :type Integer) (bFromSweep :type Boolean) (SweepResult :type "HitResult Structure (by ref)"))
  (bind _asside_scroller_character (cast `/Game/SideScrollerBP/Blueprints/SideScrollerCharacter` OtherActor))
  (`/Game/SideScrollerBP/Blueprints/SideScrollerCharacter.Death` _asside_scroller_character))

(fn `UserConstructionScript`
  (`SceneComponent.K2_AttachToComponent` (`self.NS_SpiderSlime`) (`self.SkeletalMesh`) "Head" "SnapToTarget" "SnapToTarget" "SnapToTarget" true))