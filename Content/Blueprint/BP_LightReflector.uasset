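; BP_LightReflector is an interactable reflector that rotates its mesh to redirect light, apparently for a light-beam mechanic.
; Interact passes a DoOnce gate and plays a timeline that rolls the mesh from its stored rotation.
; On finish it saves the new rotation, has each lit entry in LightScource recast its light, and resets the gate per entry.
; The dynamic-material emission code is disconnected.
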(event `self.ReceiveBeginPlay`)

(event `/Game/Blueprint/BPI_Interact.Interact`
  (params (Player :type "/Game/SideScrollerBP/Blueprints/SideScrollerCharacter Object Reference"))
  (`/Engine/EditorBlueprintResources/StandardMacros.DoOnce` false :!label _label
    (:`Completed`
      (bind (_direction _rotatetrack) (`Timeline|RotateTimeline` :!via `PlayFromStart`)
        (:`Update`
          (bind _returnvalue (+ _rotatetrack (`self.CurrentRotation`)))
          (`SceneComponent.K2_SetRelativeRotation` (`self.StaticMesh`) (`KismetMathLibrary.MakeRotator` _returnvalue) false false))
        (:`Finished`
          (set `self.CurrentRotation` _returnvalue)
          (for _array_element (`self.LightScource`)
            (if (`/Game/Blueprint/BP_laser.LightOn?` _array_element)
              (`/Game/Blueprint/BP_laser.CastLight` _array_element)
              (goto _label :!via `Reset`)
              (else
                (goto _label :!via `Reset`)))))))))

(fn `UserConstructionScript`)