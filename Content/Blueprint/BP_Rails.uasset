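; BP_Rails is an editor-built actor that lays out a repeated row of rail meshes.
; Its construction script assigns the Rails_1 mesh to the instanced Rails component, then loops from zero to NumberOfRails, adding instances along local Y spaced by GapBetweenRails.
; The component's location and the gap value are each set to themselves, and the event graph has no active logic.
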(fn `UserConstructionScript`
  (bind _rails (`self.Rails`))
  (bind (_returnvalue_x _returnvalue_y _returnvalue_z) (`KismetMathLibrary.BreakVector` (`SceneComponent.K2_GetComponentLocation` _rails)))
  (`SceneComponent.K2_SetWorldLocation` _rails (`KismetMathLibrary.MakeVector` _returnvalue_x _returnvalue_y _returnvalue_z) false false)
  (`StaticMeshComponent.SetStaticMesh` (`self.Rails`) "/Game/Teammates/Joseph/Rails_1.Rails_1")
  (set `self.GapBetweenRails` (`self.GapBetweenRails`))
  (for _index (range (+ (`self.NumberOfRails`) 1))
    (`InstancedStaticMeshComponent.AddInstance` (`self.Rails`) (`KismetMathLibrary.MakeTransform` (`KismetMathLibrary.MakeVector` 0.0 (`KismetMathLibrary.Conv_IntToDouble` (* _index (`self.GapBetweenRails`))))))))