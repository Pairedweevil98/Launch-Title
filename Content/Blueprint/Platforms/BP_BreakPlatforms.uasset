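; Breakable platform that drops out from under the player and respawns after a delay.
; When the player character overlaps the Box, the Brake timeline moves the Cube along local Z, then enables physics simulation on it so it falls.
; After the delay, Respawn turns physics off and returns the Cube to the world location saved at BeginPlay, with default rotation and its current scale.
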(event `self.ReceiveBeginPlay`
  (set `self.WorldLoc` (`SceneComponent.K2_GetComponentLocation` (`self.Cube`))))

(event `self.Box.OnComponentBeginOverlap`
  (params (OverlappedComponent :type "PrimitiveComponent Object Reference") (OtherActor :type "Actor Object Reference") (OtherComp :type "PrimitiveComponent Object Reference") (OtherBodyIndex :type Integer) (bFromSweep :type Boolean) (SweepResult :type "HitResult Structure (by ref)"))
  (if (== OtherActor (`GameplayStatics.GetPlayerCharacter` 0))
    (bind (_direction _moveupdown) (`Timeline|Brake` :!via `PlayFromStart`)
      (:`Update`
        (`SceneComponent.K2_SetRelativeLocation` (`self.Cube`) (`KismetMathLibrary.MakeVector` 0.0 0.0 (`KismetMathLibrary.Lerp` 25.0 -25.0 _moveupdown)) false false))
      (:`Finished`
        (`PrimitiveComponent.SetSimulatePhysics` (`self.Cube`) true)
        (`KismetSystemLibrary.Delay` 10.0)
        (`self.Respawn`)))))

(event `Respawn`
  (bind _cube (`self.Cube`))
  (`PrimitiveComponent.SetSimulatePhysics` _cube false)
  (`SceneComponent.K2_SetWorldTransform` _cube (`KismetMathLibrary.MakeTransform` (`self.WorldLoc`) (struct) (`SceneComponent.K2_GetComponentScale` _cube)) false false))

(fn `UserConstructionScript`)