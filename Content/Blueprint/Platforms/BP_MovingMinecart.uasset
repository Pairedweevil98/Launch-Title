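; BP_MovingMinecart is a moving minecart platform that rides along a spline when the player character enters its trigger box.
; A DoOnce gates the MoveUpDown timeline, whose play rate comes from Duration, and rearms when the ride finishes.
; Timeline updates place the platform along the spline, map spline pitch to its roll, and spin both wheels.
; PlayerDeath waits briefly, restarts then immediately stops the timeline, and rearms the trigger.
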(event `self.ReceiveBeginPlay`
  (`TimelineComponent.SetPlayRate` (`self.MoveUp/Down`) (/ 1.0 (`self.Duration`))))

(event `/Game/Blueprint/BPI_Death.PlayerDeath`
  (bind _spline (`self.Spline`))
  (`KismetSystemLibrary.Delay` 1.0)
  (`|ExecutionSequence`
    (:`then_0`
      (bind (_direction _movetrack) (`Timeline|MoveUp/Down` :!via `PlayFromStart` :!label _label)
        (:`Update`
          (bind _returnvalue (`KismetMathLibrary.Lerp` 0.0 (`SplineComponent.GetSplineLength` _spline) _movetrack))
          (`SceneComponent.K2_SetWorldLocation` (`self.Platform`) (`SplineComponent.GetLocationAtDistanceAlongSpline` (`self.Spline`) _returnvalue "World") false false)
          (bind (_returnvalue_roll _returnvalue_pitch) (`KismetMathLibrary.BreakRotator` (`SplineComponent.GetRotationAtDistanceAlongSpline` _spline _returnvalue "Local")))
          (`SceneComponent.K2_SetWorldRotation` (`self.Platform`) (`KismetMathLibrary.MakeRotator` _returnvalue_pitch) false false)
          (`SceneComponent.K2_SetWorldRotation` (`self.Wheel`) (`KismetMathLibrary.MakeRotator` (* _movetrack -10000.0)) false false)
          (`SceneComponent.K2_SetWorldRotation` (`self.Wheel1`) (`KismetMathLibrary.MakeRotator` (* _movetrack -10000.0)) false false))
        (:`Finished`
          (goto _label_2 :!via `Reset`))))
    (:`then_1`
      (goto _label :!via `Stop`))
    (:`then_2`
      (goto _label_2 :!via `Reset`))))

(event `self.Box.OnComponentBeginOverlap`
  (params (OverlappedComponent :type "PrimitiveComponent Object Reference") (OtherActor :type "Actor Object Reference") (OtherComp :type "PrimitiveComponent Object Reference") (OtherBodyIndex :type Integer) (bFromSweep :type Boolean) (SweepResult :type "HitResult Structure (by ref)"))
  (if (== OtherActor (`GameplayStatics.GetPlayerCharacter` 0))
    (`/Engine/EditorBlueprintResources/StandardMacros.DoOnce` false :!label _label_2
      (:`Completed`
        (goto _label)))))

(event `self.Box.OnComponentEndOverlap`
  (params (OverlappedComponent :type "PrimitiveComponent Object Reference") (OtherActor :type "Actor Object Reference") (OtherComp :type "PrimitiveComponent Object Reference") (OtherBodyIndex :type Integer))
  (if (== OtherActor (`GameplayStatics.GetPlayerCharacter` 0))
    _))

(fn `UserConstructionScript`)