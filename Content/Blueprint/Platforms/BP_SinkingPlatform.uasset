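; BP_SinkingPlatform is a platform that sinks while the player stands in its Box trigger and rises again after they leave.
; On begin overlap, a timeline plays and lerps the Sphere component's relative Z downward.
; On end overlap, the timeline stops, then reverses after a short delay, which re-entering the trigger does not cancel.
; Both overlap events respond only to player character 0.
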(event `self.Box.OnComponentBeginOverlap`
  (params (OverlappedComponent :type "PrimitiveComponent Object Reference") (OtherActor :type "Actor Object Reference") (OtherComp :type "PrimitiveComponent Object Reference") (OtherBodyIndex :type Integer) (bFromSweep :type Boolean) (SweepResult :type "HitResult Structure (by ref)"))
  (if (== OtherActor (`GameplayStatics.GetPlayerCharacter` 0))
    (bind (_direction _alpha) (`Timeline|SinkingTL` :!label _label)
      (:`Update`
        (`SceneComponent.K2_SetRelativeLocation` (`self.Sphere`) (`KismetMathLibrary.MakeVector` 0.0 0.0 (`KismetMathLibrary.Lerp` 0.0 -50.0 _alpha)) false false)))))

(event `self.Box.OnComponentEndOverlap`
  (params (OverlappedComponent :type "PrimitiveComponent Object Reference") (OtherActor :type "Actor Object Reference") (OtherComp :type "PrimitiveComponent Object Reference") (OtherBodyIndex :type Integer))
  (if (== OtherActor (`GameplayStatics.GetPlayerCharacter` 0))
    (`|ExecutionSequence`
      (:`then_0`
        (goto _label :!via `Stop`))
      (:`then_1`
        (`KismetSystemLibrary.Delay` 0.5)
        (goto _label :!via `Reverse`)))))

(fn `UserConstructionScript`)