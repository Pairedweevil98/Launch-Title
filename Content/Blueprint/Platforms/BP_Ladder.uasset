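; BP_Ladder is a climbable ladder platform for the side-scroller character.
; Its construction script pins the actor to a fixed X plane, stacks mesh segments to LadderHeight and fits the trigger Box to them.
; Overlap sets the character's OnLadder flag and switches player 0 to Flying if a forward trace hits this ladder.
; Leaving clears the flag and sets player 0 to Falling.
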(event `self.Box.OnComponentBeginOverlap`
  (params (OverlappedComponent :type "PrimitiveComponent Object Reference") (OtherActor :type "Actor Object Reference") (OtherComp :type "PrimitiveComponent Object Reference") (OtherBodyIndex :type Integer) (bFromSweep :type Boolean) (SweepResult :type "HitResult Structure (by ref)"))
  (bind _returnvalue (`GameplayStatics.GetPlayerCharacter` 0))
  (bind _returnvalue_2 (`self.K2_GetActorLocation` _returnvalue))
  (bind _asside_scroller_character (cast `/Game/SideScrollerBP/Blueprints/SideScrollerCharacter` OtherActor))
  (set `/Game/SideScrollerBP/Blueprints/SideScrollerCharacter.OnLadder?` true _asside_scroller_character)
  (bind _outhit (`KismetSystemLibrary.LineTraceSingle` :`Start` _returnvalue_2 :`End` (+ _returnvalue_2 (* (`self.GetActorForwardVector` _returnvalue) 500.0)) :`TraceChannel` "TraceTypeQuery1" :`bIgnoreSelf` false))
  (if (== (`.HitActor` (`GameplayStatics.BreakHitResult` _outhit)) self)
    (`CharacterMovementComponent.SetMovementMode` (`Character.CharacterMovement` (`GameplayStatics.GetPlayerCharacter` 0)) "MOVE_Flying" 0)))

(event `self.Box.OnComponentEndOverlap`
  (params (OverlappedComponent :type "PrimitiveComponent Object Reference") (OtherActor :type "Actor Object Reference") (OtherComp :type "PrimitiveComponent Object Reference") (OtherBodyIndex :type Integer))
  (bind _asside_scroller_character (cast `/Game/SideScrollerBP/Blueprints/SideScrollerCharacter` OtherActor))
  (set `/Game/SideScrollerBP/Blueprints/SideScrollerCharacter.OnLadder?` false _asside_scroller_character)
  (`CharacterMovementComponent.SetMovementMode` (`Character.CharacterMovement` (`GameplayStatics.GetPlayerCharacter` 0)) "MOVE_Falling" 0))

(fn `UserConstructionScript`
  (bind (_relativelocation_x _relativelocation_y _relativelocation_z) (`KismetMathLibrary.BreakVector` (`SceneComponent.RelativeLocation` (`self.DefaultSceneRoot`))))
  (`self.K2_SetActorLocation` (`KismetMathLibrary.MakeVector` 1200.0 _relativelocation_y _relativelocation_z))
  (for _index (range (+ (`KismetMathLibrary.FTrunc` (/ (`self.LadderHeight`) 550.0)) 1))
    (`AddComponent|NODE_AddStaticMeshComponent-0` :`RelativeTransform` (`KismetMathLibrary.MakeTransform` (`KismetMathLibrary.MakeVector` 0.0 0.0 (* _index 550.0)))))
  (`SceneComponent.K2_SetRelativeLocation` (`self.Box`) (`KismetMathLibrary.MakeVector` 0.0 0.0 (+ (/ (`self.LadderHeight`) 2.0) -200.0)) false false)
  (`BoxComponent.SetBoxExtent` (`self.Box`) (`KismetMathLibrary.MakeVector` 64.0 32.0 (- (/ (`self.LadderHeight`) 2.0) 50.0)) true))