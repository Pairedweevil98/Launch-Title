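; Falling spike trap for a side-scroller that drops when the player enters its trigger box and kills characters touching its hit box.
; The trigger, positioned per instance by the construction script, fires once, switching off the particle effect and chaining wiggle and fall timelines on the cone, then shaking the camera.
; On PlayerDeath, after a short delay, it re-arms the trigger and restarts then immediately stops the fall timeline to rewind the spike.
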(event `self.Box.OnComponentBeginOverlap`
  (params (OverlappedComponent :type "PrimitiveComponent Object Reference") (OtherActor :type "Actor Object Reference") (OtherComp :type "PrimitiveComponent Object Reference") (OtherBodyIndex :type Integer) (bFromSweep :type Boolean) (SweepResult :type "HitResult Structure (by ref)"))
  (if (== OtherActor (`GameplayStatics.GetPlayerCharacter` 0))
    (`/Engine/EditorBlueprintResources/StandardMacros.DoOnce` false :!label _label
      (:`Completed`
        (`ActorComponent.SetActive` (`self.NS_FallingSpike`) false false)
        (bind (_direction _alpha) (`Timeline|WiggleTL`)
          (:`Update`
            (`SceneComponent.K2_SetRelativeRotation` (`self.Cone`) (`KismetMathLibrary.MakeRotator` (`KismetMathLibrary.Lerp` 5.0 -5.0 _alpha) 180.0) false false))
          (:`Finished`
            (bind (_direction_2 _alpha_2) (`Timeline|FallingTL` :!label _label_2)
              (:`Update`
                (bind (_returnvalue_x _returnvalue_y _returnvalue_z) (`KismetMathLibrary.BreakVector` (`KismetMathLibrary.VLerp` (0.0 0.0 0.0) (`self.FallLoc`) _alpha_2)))
                (`SceneComponent.K2_SetRelativeLocation` (`self.Cone`) (`KismetMathLibrary.MakeVector` 0.0 0.0 _returnvalue_z) false false))
              (:`Finished`
                (`GameplayStatics.PlayWorldCameraShake` "/Game/Blueprint/Camera/FallingSpikeCamShake.FallingSpikeCamShake_C" (`SceneComponent.K2_GetComponentLocation` (`self.Cone`)) 0.0 5000.0)))))))))

(event `/Game/Blueprint/BPI_Death.PlayerDeath`
  (`KismetSystemLibrary.Delay` 1.0)
  (`|ExecutionSequence`
    (:`then_0`
      (goto _label :!via `Reset`))
    (:`then_1`
      (goto _label_2 :!via `PlayFromStart`))
    (:`then_2`
      (goto _label_2 :!via `Stop`))))

(event `self.Box1.OnComponentBeginOverlap`
  (params (OverlappedComponent :type "PrimitiveComponent Object Reference") (OtherActor :type "Actor Object Reference") (OtherComp :type "PrimitiveComponent Object Reference") (OtherBodyIndex :type Integer) (bFromSweep :type Boolean) (SweepResult :type "HitResult Structure (by ref)"))
  (bind _asside_scroller_character (cast `/Game/SideScrollerBP/Blueprints/SideScrollerCharacter` OtherActor))
  (`/Game/SideScrollerBP/Blueprints/SideScrollerCharacter.Death` _asside_scroller_character))

(fn `UserConstructionScript`
  (`SceneComponent.K2_SetRelativeTransform` (`self.Box`) (`self.BoxCollisionTransform`) false false))