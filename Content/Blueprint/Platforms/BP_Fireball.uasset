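; BP_Fireball is a side-scroller hazard that moves a fireball vertically and kills the player character on contact.
; On BeginPlay, the Selection value picks a start delay, allowing instances to be staggered.
; A timeline then drives the Fireball component's relative Z between zero and Height through a Lerp.
; Overlapping the Sphere component calls Death on a SideScrollerCharacter.
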(event `self.ReceiveBeginPlay`
  (switch `/Game/Blueprint/Platforms/FireBallTimeings` (`self.Selection`)
    (:`NewEnumerator0`
      (set `self.Duration` (`self.1Sec`)))
    (:`NewEnumerator1`
      (set `self.Duration` (`self.2Sec`)))
    (:`NewEnumerator2`
      (set `self.Duration` (`self.3Sec`))))
  (`KismetSystemLibrary.Delay` (`self.Duration`))
  (bind (_direction _alpha_) (`Timeline|FireBallTL`)
    (:`Update`
      (`SceneComponent.K2_SetRelativeLocation` (`self.Fireball`) (`KismetMathLibrary.MakeVector` 0.0 0.0 (`KismetMathLibrary.Lerp` 0.0 (`self.Height`) _alpha_)) false false))))

(event `self.Sphere.OnComponentBeginOverlap`
  (params (OverlappedComponent :type "PrimitiveComponent Object Reference") (OtherActor :type "Actor Object Reference") (OtherComp :type "PrimitiveComponent Object Reference") (OtherBodyIndex :type Integer) (bFromSweep :type Boolean) (SweepResult :type "HitResult Structure (by ref)"))
  (bind _asside_scroller_character (cast `/Game/SideScrollerBP/Blueprints/SideScrollerCharacter` OtherActor))
  (`/Game/SideScrollerBP/Blueprints/SideScrollerCharacter.Death` _asside_scroller_character))

(fn `UserConstructionScript`)