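; TestLever is an interactable platform lever that raises and lowers a linked MoveableTrack when powered.
; Interact plays a pull sound, then a FlipFlop alternates between moving the track up and down, playing or reversing a timeline that tilts the handle.
; A text render shows the powered state, set at construction and by SetPowered, which updates only the text and leaves the Powered variable untouched.
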(event `SetPowered`
  (params (`On/Off` :type Boolean))
  (bind _textrender (`self.TextRender`))
  (if `On/Off`
    (`TextRenderComponent.K2_SetText` _textrender (`self.PoweredOn`))
    (else
      (`TextRenderComponent.K2_SetText` _textrender (`self.PoweredOff`)))))

(event `/Game/Blueprint/BPI_Interact.Interact`
  (params (Player :type "/Game/SideScrollerBP/Blueprints/SideScrollerCharacter Object Reference"))
  (bind _moveabletrack (`self.MoveableTrack`))
  (if (`self.Powered`)
    (`AudioComponent.Play` (`self.LevelPull_Cue`) 0.0)
    (`/Engine/EditorBlueprintResources/StandardMacros.FlipFlop`
      (:`A`
        (`/Game/Blueprint/Platforms/TestMoveableTrack.MoveUp` _moveabletrack)
        (bind (_direction _rotatelever) (`Timeline|MoveLever` :!label _label)
          (:`Update`
            (`SceneComponent.K2_SetRelativeRotation` (`self.LeverHandle`) (`KismetMathLibrary.MakeRotator` (`KismetMathLibrary.Lerp` 45.0 -45.0 _rotatelever)) false false))))
      (:`B`
        (`/Game/Blueprint/Platforms/TestMoveableTrack.MoveDown` _moveabletrack)
        (goto _label :!via `Reverse`)))))

(fn `UserConstructionScript`
  (bind _textrender (`self.TextRender`))
  (if (`self.Powered`)
    (`TextRenderComponent.K2_SetText` _textrender (`self.PoweredOn`))
    (else
      (`TextRenderComponent.K2_SetText` _textrender (`self.PoweredOff`)))))