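; Interactable climbable ladder, built in the construction script from stacked mesh segments with a box volume sized to LadderHeight.
; Interact toggles the player's OnLadder state: mounting sets Flying movement and snaps the character to the ladder's Y, dismounting restores Falling and orient-to-movement.
; While mounted, a delayed while-loop macro keeps reapplying a fixed facing with orient-to-movement disabled.
; Leaving the box also dismounts the player.
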(event `/Game/Blueprint/BPI_Interact.Interact`
  (params (Player :type "/Game/SideScrollerBP/Blueprints/SideScrollerCharacter Object Reference"))
  (bind (_returnvalue_x _returnvalue_y) (`KismetMathLibrary.BreakVector` (`self.K2_GetActorLocation`)))
  (bind _returnvalue (`GameplayStatics.GetPlayerCharacter` 0))
  (bind _player (`self.Player`))
  (bind (_returnvalue_x_2 _returnvalue_y_2 _returnvalue_z) (`KismetMathLibrary.BreakVector` (`self.K2_GetActorLocation` _returnvalue)))
  (bind _output_get (set `self.Player` Player))
  (if (`/Game/SideScrollerBP/Blueprints/SideScrollerCharacter.OnLadder?` _output_get)
    (if (`/Game/SideScrollerBP/Blueprints/SideScrollerCharacter.OnLadder?` _player) :!label _label
      (set `/Game/SideScrollerBP/Blueprints/SideScrollerCharacter.OnLadder?` false _player)
      (`CharacterMovementComponent.SetMovementMode` (`Character.CharacterMovement` (`GameplayStatics.GetPlayerCharacter` 0)) "MOVE_Falling" 0)
      (set `CharacterMovementComponent.bOrientRotationToMovement` true (`Character.CharacterMovement` (`GameplayStatics.GetPlayerCharacter` 0))))
    (else
      (bind _output_get_2 (set `/Game/SideScrollerBP/Blueprints/SideScrollerCharacter.OnLadder?` true _output_get))
      (if _output_get_2
        (`CharacterMovementComponent.SetMovementMode` (`Character.CharacterMovement` (`GameplayStatics.GetPlayerCharacter` 0)) "MOVE_Flying" 0)
        (`self.K2_TeleportTo` :`self` _returnvalue :`DestLocation` (`KismetMathLibrary.MakeVector` _returnvalue_x_2 _returnvalue_y _returnvalue_z))
        (`self.WhileLoopWithDelay` (`/Game/SideScrollerBP/Blueprints/SideScrollerCharacter.OnLadder?` (`self.Player`))
          (:`LoopBody`
            (`self.K2_SetActorRotation` _returnvalue (`KismetMathLibrary.MakeRotator` 0.0 0.0 180.0) false)
            (set `CharacterMovementComponent.bOrientRotationToMovement` false (`Character.CharacterMovement` (`GameplayStatics.GetPlayerCharacter` 0)))))))))

(event `self.Box.OnComponentEndOverlap`
  (params (OverlappedComponent :type "PrimitiveComponent Object Reference") (OtherActor :type "Actor Object Reference") (OtherComp :type "PrimitiveComponent Object Reference") (OtherBodyIndex :type Integer))
  (`/Engine/EditorBlueprintResources/StandardMacros.IsValid` (`self.Player`)
    (:`Is Valid`
      (goto _label))))

(fn `UserConstructionScript`
  (for _index (range (+ (`KismetMathLibrary.FTrunc` (/ (`self.LadderHeight`) 70.0)) 1))
    (`AddComponent|NODE_AddStaticMeshComponent-0` :`RelativeTransform` (`KismetMathLibrary.MakeTransform` (`KismetMathLibrary.MakeVector` 0.0 0.0 (* _index 70.0)))))
  (`SceneComponent.K2_SetRelativeLocation` (`self.Box`) (`KismetMathLibrary.MakeVector` 0.0 0.0 (+ (/ (`self.LadderHeight`) 2.0) 0.0)) false false)
  (`BoxComponent.SetBoxExtent` (`self.Box`) (`KismetMathLibrary.MakeVector` 64.0 32.0 (- (/ (`self.LadderHeight`) 2.0) -30.0)) true))