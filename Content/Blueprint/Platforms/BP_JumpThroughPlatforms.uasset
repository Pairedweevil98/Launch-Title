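; One-way jump-through platform that the player can rise through from below and then stand on.
; The platform ignores Pawn collision until the player character overlaps its Box, then blocks immediately if the player's mesh origin is higher, or after a short delay otherwise.
; Leaving the Box restores Ignore for the Pawn channel.
; The construction script snaps the root to a fixed world X, keeping instances on one plane.
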(event `self.ReceiveBeginPlay`
  (`PrimitiveComponent.SetCollisionResponseToChannel` (`self.Platform`) "ECC_Pawn" "ECR_Ignore"))

(event `self.Box.OnComponentBeginOverlap`
  (params (OverlappedComponent :type "PrimitiveComponent Object Reference") (OtherActor :type "Actor Object Reference") (OtherComp :type "PrimitiveComponent Object Reference") (OtherBodyIndex :type Integer) (bFromSweep :type Boolean) (SweepResult :type "HitResult Structure (by ref)"))
  (bind _returnvalue (`GameplayStatics.GetPlayerCharacter` 0))
  (bind (_returnvalue_x _returnvalue_y _returnvalue_z) (`KismetMathLibrary.BreakVector` (`SceneComponent.K2_GetComponentLocation` (`self.Platform`))))
  (bind (_returnvalue_x_2 _returnvalue_y_2 _returnvalue_z_2) (`KismetMathLibrary.BreakVector` (`SceneComponent.K2_GetComponentLocation` (`Character.Mesh` _returnvalue))))
  (if (== OtherActor _returnvalue)
    (if (not (> _returnvalue_z_2 _returnvalue_z))
      (`KismetSystemLibrary.Delay` 0.2))
    (`PrimitiveComponent.SetCollisionResponseToChannel` (`self.Platform`) "ECC_Pawn" "ECR_Block")))

(event `self.Box.OnComponentEndOverlap`
  (params (OverlappedComponent :type "PrimitiveComponent Object Reference") (OtherActor :type "Actor Object Reference") (OtherComp :type "PrimitiveComponent Object Reference") (OtherBodyIndex :type Integer))
  (if (== OtherActor (`GameplayStatics.GetPlayerCharacter` 0))
    (`PrimitiveComponent.SetCollisionResponseToChannel` (`self.Platform`) "ECC_Pawn" "ECR_Ignore")))

(fn `UserConstructionScript`
  (bind _defaultsceneroot (`self.DefaultSceneRoot`))
  (bind (_returnvalue_x _returnvalue_y _returnvalue_z) (`KismetMathLibrary.BreakVector` (`SceneComponent.K2_GetComponentLocation` _defaultsceneroot)))
  (`SceneComponent.K2_SetWorldLocation` _defaultsceneroot (`KismetMathLibrary.MakeVector` 1200.0 _returnvalue_y _returnvalue_z) false false))