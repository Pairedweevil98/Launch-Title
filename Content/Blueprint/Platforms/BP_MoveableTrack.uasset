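; BP_MoveableTrack is a track platform that moves between two relative locations, carrying an overlapping minecart with it.
; MoveUp and MoveDown play and reverse a Duration-scaled timeline that lerps the platform and cart.
; A box overlap caches the BP_Minecart and sets its Overlapping flag, clearing it after a short retriggerable delay on exit.
; MoveUp captures cart endpoints through a DoOnce, offsetting by the platform's travel, and resets it when no cart overlaps.
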(event `self.ReceiveBeginPlay`
  (`TimelineComponent.SetPlayRate` (`self.MoveUp/Down`) (/ 1.0 (`self.Duration`))))

(event `MoveUp`
  (`self.SetCartStart/End`)
  (bind (_direction _movetrack) (`Timeline|MoveUp/Down` :!label _label)
    (:`Update`
      (`SceneComponent.K2_SetRelativeLocation` (`self.Platform`) (`KismetMathLibrary.VLerp` (`self.Loc1`) (`self.Loc2`) _movetrack) false false)
      (bind _bp_minecart (`self.BP_Minecart`)
        (:`then`
          (if (`/Game/Blueprint/Puzzles/BP_Pushable.Overlapping?` _bp_minecart)
            (`self.K2_SetActorLocation` _bp_minecart (`KismetMathLibrary.VLerp` (`self.MinecartStart`) (`self.MinecartEnd`) _movetrack) false false)))
        (:`else`)))))

(event `MoveDown`
  (goto _label :!via `Reverse`))

(event `self.Box.OnComponentBeginOverlap`
  (params (OverlappedComponent :type "PrimitiveComponent Object Reference") (OtherActor :type "Actor Object Reference") (OtherComp :type "PrimitiveComponent Object Reference") (OtherBodyIndex :type Integer) (bFromSweep :type Boolean) (SweepResult :type "HitResult Structure (by ref)"))
  (`/Engine/EditorBlueprintResources/StandardMacros.IsValid` (`self.BP_Minecart`)
    (:`Is Valid`
      _)
    (:`Is Not Valid`
      (bind _asbp_minecart (cast `/Game/Blueprint/Puzzles/BP_Minecart` OtherActor))
      (set `self.BP_Minecart` _asbp_minecart)))
  (if (== OtherActor (`self.BP_Minecart`))
    (set `/Game/Blueprint/Puzzles/BP_Pushable.Overlapping?` true (`self.BP_Minecart`))))

(event `SetCartStart/End`
  (if (`/Game/Blueprint/Puzzles/BP_Pushable.Overlapping?` (`self.BP_Minecart`))
    (`/Engine/EditorBlueprintResources/StandardMacros.DoOnce` false :!label _label_2
      (:`Completed`
        (bind _output_get (set `self.MinecartStart` (`self.K2_GetActorLocation` (`self.BP_Minecart`))))
        (set `self.MinecartEnd` (+ _output_get (- (`self.Loc2`) (`self.Loc1`))))))
    (else
      (goto _label_2 :!via `Reset`))))

(event `self.Box.OnComponentEndOverlap`
  (params (OverlappedComponent :type "PrimitiveComponent Object Reference") (OtherActor :type "Actor Object Reference") (OtherComp :type "PrimitiveComponent Object Reference") (OtherBodyIndex :type Integer))
  (if (== OtherActor (`self.BP_Minecart`))
    (`KismetSystemLibrary.RetriggerableDelay` 0.2)
    (set `/Game/Blueprint/Puzzles/BP_Pushable.Overlapping?` false (`self.BP_Minecart`))))

(fn `UserConstructionScript`)