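; A platform actor that travels along a spline and carries a minecart with it.
; MoveUp and MoveDown play and reverse a Duration-scaled timeline that positions Platform by distance along the spline.
; Box overlaps cache the BP_Minecart and set its Overlapping flag, clearing it after a retriggerable delay.
; While moving, an overlapping cart attaches once to Box, then detaches and re-arms when the timeline finishes.
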(event `self.ReceiveBeginPlay`
  (`TimelineComponent.SetPlayRate` (`self.MoveUp/Down`) (/ 1.0 (`self.Duration`))))

(event `MoveUp`
  (bind (_direction _movetrack) (`Timeline|MoveUp/Down` :!label _label)
    (:`Update`
      (`SceneComponent.K2_SetWorldLocation` (`self.Platform`) (`SplineComponent.GetLocationAtDistanceAlongSpline` (`self.Spline`) (`KismetMathLibrary.Lerp` 0.0 (`SplineComponent.GetSplineLength` (`self.Spline`)) _movetrack) "World") false false)
      (`/Engine/EditorBlueprintResources/StandardMacros.IsValid` (`self.BP_Minecart`)
        (:`Is Valid`
          (if (`/Game/Blueprint/Puzzles/BP_Pushable.Overlapping?` (`self.BP_Minecart`))
            (`/Engine/EditorBlueprintResources/StandardMacros.DoOnce` false :!label _label_2
              (:`Completed`
                (`self.K2_AttachToComponent` (`self.BP_Minecart`) (`self.Box`) "None" "KeepWorld" "KeepWorld" "KeepWorld" true)))))))
    (:`Finished`
      (`self.Detach`))))

(event `MoveDown`
  (goto _label :!via `Reverse`))

(event `Detach`
  (`/Engine/EditorBlueprintResources/StandardMacros.IsValid` (`self.BP_Minecart`)
    (:`Is Valid`
      (if (`/Game/Blueprint/Puzzles/BP_Pushable.Overlapping?` (`self.BP_Minecart`))
        (`self.K2_DetachFromActor` (`self.BP_Minecart`) "KeepWorld" "KeepWorld" "KeepWorld")
        (goto _label_2 :!via `Reset`)))))

(event `self.Box.OnComponentBeginOverlap`
  (params (OverlappedComponent :type "PrimitiveComponent Object Reference") (OtherActor :type "Actor Object Reference") (OtherComp :type "PrimitiveComponent Object Reference") (OtherBodyIndex :type Integer) (bFromSweep :type Boolean) (SweepResult :type "HitResult Structure (by ref)"))
  (`/Engine/EditorBlueprintResources/StandardMacros.IsValid` (`self.BP_Minecart`)
    (:`Is Valid`
      _)
    (:`Is Not Valid`
      (bind _asbp_minecart (cast `/Game/Blueprint/Puzzles/BP_Minecart` OtherActor))
      (set `self.BP_Minecart` _asbp_minecart)))
  (if (== OtherActor (`self.BP_Minecart`))
    (set `/Game/Blueprint/Puzzles/BP_Pushable.Overlapping?` true (`self.BP_Minecart`))))

(event `self.Box.OnComponentEndOverlap`
  (params (OverlappedComponent :type "PrimitiveComponent Object Reference") (OtherActor :type "Actor Object Reference") (OtherComp :type "PrimitiveComponent Object Reference") (OtherBodyIndex :type Integer))
  (if (== OtherActor (`self.BP_Minecart`))
    (`KismetSystemLibrary.RetriggerableDelay` 0.2)
    (set `/Game/Blueprint/Puzzles/BP_Pushable.Overlapping?` false (`self.BP_Minecart`))))

(fn `UserConstructionScript`)