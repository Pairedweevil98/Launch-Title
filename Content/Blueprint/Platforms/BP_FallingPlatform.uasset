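; BP_FallingPlatform is a platform that shakes, falls and resets after the player enters its Box trigger.
; A DoOnce-gated overlap chains two timelines: TLMoving wobbles the actor vertically, then TLFall moves it downward.
; Each update offsets Z from the StaticMesh's current relative location rather than the cached start.
; After a delay, the actor returns to the mesh location saved at BeginPlay and rearms the trigger.
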(event `self.ReceiveBeginPlay`
  (set `self.Location` (`SceneComponent.K2_GetComponentLocation` (`self.StaticMesh`))))

(event `self.Box.OnComponentBeginOverlap`
  (params (OverlappedComponent :type "PrimitiveComponent Object Reference") (OtherActor :type "Actor Object Reference") (OtherComp :type "PrimitiveComponent Object Reference") (OtherBodyIndex :type Integer) (bFromSweep :type Boolean) (SweepResult :type "HitResult Structure (by ref)"))
  (bind (_relativelocation_x _relativelocation_y _relativelocation_z) (`KismetMathLibrary.BreakVector` (`SceneComponent.RelativeLocation` (`self.StaticMesh`))))
  (bind (_relativelocation_x_2 _relativelocation_y_2 _relativelocation_z_2) (`KismetMathLibrary.BreakVector` (`SceneComponent.RelativeLocation` (`self.StaticMesh`))))
  (if (== OtherActor (`GameplayStatics.GetPlayerCharacter` 0))
    (`/Engine/EditorBlueprintResources/StandardMacros.DoOnce` false :!label _label
      (:`Completed`
        (bind (_direction _alpha) (`Timeline|TLMoving` :!via `PlayFromStart`)
          (:`Update`
            (`self.K2_SetActorRelativeLocation` (`KismetMathLibrary.MakeVector` _relativelocation_x_2 _relativelocation_y_2 (+ _relativelocation_z_2 (`KismetMathLibrary.Lerp` -2.0 2.0 _alpha)))))
          (:`Finished`
            (bind (_direction_2 _alpha_2) (`Timeline|TLFall` :!via `PlayFromStart`)
              (:`Update`
                (`self.K2_SetActorRelativeLocation` (`KismetMathLibrary.MakeVector` _relativelocation_x _relativelocation_y (+ _relativelocation_z (`KismetMathLibrary.Lerp` 0.0 -100.0 _alpha_2)))))
              (:`Finished`
                (`KismetSystemLibrary.Delay` 5.0)
                (`self.K2_SetActorLocation` (`self.Location`))
                (goto _label :!via `Reset`)))))))))

(fn `UserConstructionScript`)