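; Character component that lets the side-scroller character push and pull pushable actors.
; BeginPush attaches the character to the object, constrains its movement plane and enables Tick; EndPush reverses this.
; Tick reads A/D directly, using relative Y position to choose push or pull, sweeps the object along the character's forward axis, sets Pulling/PushWhileMove flags and triggers minecart light casting.
; Helpers report pushing state and the object's height above the character's feet.
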(event `self.ReceiveBeginPlay`
  (`self.SetComponentTickEnabled` false))

(event `self.ReceiveTick`
  (params (DeltaSeconds :type "Float (single-precision)"))
  (bind _returnvalue (`GameplayStatics.GetPlayerController` 0))
  (bind _returnvalue_2 (`GameplayStatics.GetPlayerController` 0))
  (bind (_returnvalue_x _returnvalue_y) (`KismetMathLibrary.BreakVector` (`Actor.K2_GetActorLocation` (`self.Owning_Character`))))
  (bind _returnvalue_3 (* DeltaSeconds (`self.PushSpeed`)))
  (bind _returnvalue_4 (* DeltaSeconds (`self.PushSpeed`)))
  (bind _currentpushable (`self.CurrentPushable`)
    (:`then`
      (bind _asbp_minecart (cast `/Game/Blueprint/Puzzles/BP_Minecart` _currentpushable)
        (:`then`
          (`/Game/Blueprint/Puzzles/BP_Minecart.CastLightFromCart` _asbp_minecart))
        (:`CastFailed`
          _))
      (bind (_returnvalue_x_2 _returnvalue_y_2) (`KismetMathLibrary.BreakVector` (`Actor.K2_GetActorLocation` _currentpushable)))
      (if (> _returnvalue_y _returnvalue_y_2)
        (if (`PlayerController.IsInputKeyDown` _returnvalue "D")
          (`Actor.K2_AddActorWorldOffset` _currentpushable (* (`Actor.GetActorForwardVector` (`self.GetOwner`)) _returnvalue_4) true false)
          (bind _asside_scroller_character (cast `/Game/SideScrollerBP/Blueprints/SideScrollerCharacter` (`self.Owning_Character`)))
          (set `/Game/SideScrollerBP/Blueprints/SideScrollerCharacter.Pulling?` false _asside_scroller_character)
          (set `/Game/SideScrollerBP/Blueprints/SideScrollerCharacter.PushWhileMove` true _asside_scroller_character)
          (elif (`PlayerController.IsInputKeyDown` _returnvalue "A")
            (`Actor.K2_AddActorWorldOffset` _currentpushable (* (* (`Actor.GetActorForwardVector` (`self.GetOwner`)) -1.0) _returnvalue_4) true false)
            (bind _asside_scroller_character_2 (cast `/Game/SideScrollerBP/Blueprints/SideScrollerCharacter` (`self.Owning_Character`)))
            (set `/Game/SideScrollerBP/Blueprints/SideScrollerCharacter.Pulling?` true _asside_scroller_character_2)
            (set `/Game/SideScrollerBP/Blueprints/SideScrollerCharacter.PushWhileMove` true _asside_scroller_character_2)
            (else
              (bind _asside_scroller_character_3 (cast `/Game/SideScrollerBP/Blueprints/SideScrollerCharacter` (`self.Owning_Character`) :!label _label))
              (set `/Game/SideScrollerBP/Blueprints/SideScrollerCharacter.PushWhileMove` false _asside_scroller_character_3))))
        (elif (`PlayerController.IsInputKeyDown` _returnvalue_2 "A")
          (`Actor.K2_AddActorWorldOffset` _currentpushable (* (`Actor.GetActorForwardVector` (`self.GetOwner`)) _returnvalue_3) true false)
          (bind _asside_scroller_character_4 (cast `/Game/SideScrollerBP/Blueprints/SideScrollerCharacter` (`self.Owning_Character`)))
          (set `/Game/SideScrollerBP/Blueprints/SideScrollerCharacter.Pulling?` false _asside_scroller_character_4)
          (set `/Game/SideScrollerBP/Blueprints/SideScrollerCharacter.PushWhileMove` true _asside_scroller_character_4)
          (elif (`PlayerController.IsInputKeyDown` _returnvalue_2 "D")
            (`Actor.K2_AddActorWorldOffset` _currentpushable (* (* (`Actor.GetActorForwardVector` (`self.GetOwner`)) -1.0) _returnvalue_3) true false)
            (bind _asside_scroller_character_5 (cast `/Game/SideScrollerBP/Blueprints/SideScrollerCharacter` (`self.Owning_Character`)))
            (set `/Game/SideScrollerBP/Blueprints/SideScrollerCharacter.Pulling?` true _asside_scroller_character_5)
            (set `/Game/SideScrollerBP/Blueprints/SideScrollerCharacter.PushWhileMove` true _asside_scroller_character_5)
            (else
              (goto _label))))))
    (:`else`)))

(fn `BeginPush`
  (params (Pushable :type "/Game/Blueprint/Puzzles/BP_Pushable Object Reference"))
  (locals (OwningCharacter :type "Character Object Reference"))
  (bind _owning_character (`self.Owning_Character`))
  (bind _charactermovement (`Character.CharacterMovement` _owning_character))
  (if (not (`KismetSystemLibrary.IsValid` (`self.CurrentPushable`)))
    (bind _ascharacter (cast `Character` (`self.GetOwner`)))
    (set `self.Owning_Character` _ascharacter)
    (bind _output_get (set `self.CurrentPushable` (`local.Pushable`)))
    (`Actor.K2_AttachToActor` (`self.Owning_Character`) _output_get "None" "KeepWorld" "KeepWorld" "KeepWorld" true)
    (`MovementComponent.SetPlaneConstraintEnabled` _charactermovement true)
    (`MovementComponent.SetPlaneConstraintNormal` _charactermovement (`Actor.GetActorRightVector` _owning_character))
    (`self.SetComponentTickEnabled` true)))

(fn `EndPush`
  (locals (OwningCharacter :type "Character Object Reference"))
  (bind _currentpushable (`self.CurrentPushable`)
    (:`then`
      (if (not (`/Game/Blueprint/Puzzles/BP_Pushable.Overlapping?` _currentpushable))
        (set `self.CurrentPushable` null)
        (bind _ascharacter (cast `Character` (`self.GetOwner`)))
        (bind _output_get (set `local.OwningCharacter` _ascharacter))
        (`Actor.K2_DetachFromActor` _output_get "KeepWorld" "KeepWorld" "KeepWorld")
        (`MovementComponent.SetPlaneConstraintEnabled` (`Character.CharacterMovement` (`local.OwningCharacter`)) false)
        (`self.SetComponentTickEnabled` false)
        (`KismetSystemLibrary.PrintString` "NotOverlapping")
        (else
          (set `self.CurrentPushable` null)
          (bind _ascharacter_2 (cast `Character` (`self.GetOwner`)))
          (bind _output_get_2 (set `local.OwningCharacter` _ascharacter_2))
          (`Actor.K2_DetachFromActor` _output_get_2 "KeepWorld" "KeepWorld" "KeepWorld")
          (`MovementComponent.SetPlaneConstraintEnabled` (`Character.CharacterMovement` (`local.OwningCharacter`)) false)
          (`self.SetComponentTickEnabled` false))))
    (:`else`)))

(fn `GetPushableHeight`
  (returns (Height :type "Float (double-precision)"))
  (locals (TopOfObject :type "Float (double-precision)" :default 0.0) (FeetOfCharacter :type "Float (double-precision)" :default 0.0))
  (bind (_returnvalue_x _returnvalue_y _returnvalue_z) (`KismetMathLibrary.BreakVector` (`Actor.K2_GetActorLocation` (`self.CurrentPushable`))))
  (`|ExecutionSequence`
    (:`then_0`
      (bind _currentpushable (`self.CurrentPushable`)
        (:`then`
          (bind (_min _max) (`StaticMeshComponent.GetLocalBounds` (`/Game/Blueprint/Puzzles/BP_Pushable.StaticMesh` _currentpushable)))
          (set `local.TopOfObject` (+ (- (.z _max) (.z _min)) _returnvalue_z))
          (bind _ascharacter (cast `Character` (`self.GetOwner`)))
          (bind (_returnvalue_x_2 _returnvalue_y_2 _returnvalue_z_2) (`KismetMathLibrary.BreakVector` (`Actor.K2_GetActorLocation` _ascharacter)))
          (set `local.FeetOfCharacter` (- _returnvalue_z_2 (`CapsuleComponent.GetScaledCapsuleHalfHeight` (`Character.CapsuleComponent` _ascharacter))))
          (return (- (`local.TopOfObject`) (`local.FeetOfCharacter`))))
        (:`else`)))
    (:`then_1`
      (return 0.0))))

(fn `IsPushingObject`
  (returns (ReturnValue :type Boolean))
  (return (`KismetSystemLibrary.IsValid` (`self.CurrentPushable`))))