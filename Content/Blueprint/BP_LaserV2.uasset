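; BP_LaserV2 is a laser beam actor rendered with two Niagara effects, one for the beam and one for the impact, tinted purple and magenta on BeginPlay.
; Each Tick it line traces a short distance along its forward vector and feeds the hit location, or trace end on a miss, into the beam's LaserEnd parameter.
; The impact effect moves to the hit point and shows only when the trace is blocked.
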(event `self.ReceiveBeginPlay`
  (`FXSystemComponent.SetColorParameter` (`self.NiagaraLaser`) "Colour" (struct :`R` 0.25 :`B` 0.25 :`A` 0.06))
  (`FXSystemComponent.SetColorParameter` (`self.NiagaraLaserImpact`) "Colour" (struct :`R` 1.0 :`B` 1.0 :`A` 1.0)))

(event `self.ReceiveTick`
  (params (DeltaSeconds :type "Float (single-precision)"))
  (bind _returnvalue (`self.K2_GetActorLocation`))
  (bind _niagaralaserimpact (`self.NiagaraLaserImpact`))
  (bind _outhit (`KismetSystemLibrary.LineTraceSingle` _returnvalue (+ _returnvalue (* (`self.GetActorForwardVector`) 500.0)) "TraceTypeQuery3"))
  (`FXSystemComponent.SetVectorParameter` (`self.NiagaraLaser`) "LaserEnd" (select `bool` (`GameplayStatics.BreakHitResult` _outhit) :`false` (`.TraceEnd` (`GameplayStatics.BreakHitResult` _outhit)) :`true` (`.Location` (`GameplayStatics.BreakHitResult` _outhit))))
  (`SceneComponent.SetVisibility` _niagaralaserimpact (`GameplayStatics.BreakHitResult` _outhit) false)
  (`SceneComponent.K2_SetWorldLocation` _niagaralaserimpact (`.Location` (`GameplayStatics.BreakHitResult` _outhit)) false false))

(fn `UserConstructionScript`)