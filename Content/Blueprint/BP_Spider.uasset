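; BP_Spider is a side-scroller hazard that kills the player on touch and can be driven away with a light beam.
; Overlapping its Box calls Death on the SideScrollerCharacter.
; On OnLightInteract it waits briefly, and if the beam still hits it, the Run timeline moves it upward, then destroys it.
; The upward Lerp starts from the current Z on each update, so movement accumulates rather than covering a fixed distance.
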(event `/Game/Blueprint/BPI_LightBeamInteract.OnLightInteract`
  (params (LightBeam :type "/Game/Blueprint/Puzzles/BP_laser Object Reference"))
  (bind (_returnvalue_x _returnvalue_y _returnvalue_z) (`KismetMathLibrary.BreakVector` (`SceneComponent.K2_GetComponentLocation` (`self.DefaultSceneRoot`))))
  (`KismetSystemLibrary.Delay` 1.0)
  (if (== (`/Game/Blueprint/Puzzles/BP_laser.HitActor` LightBeam) self)
    (bind (_direction _runtrack) (`Timeline|Run`)
      (:`Update`
        (`SceneComponent.K2_SetWorldLocation` (`self.DefaultSceneRoot`) (`KismetMathLibrary.MakeVector` _returnvalue_x _returnvalue_y (`KismetMathLibrary.Lerp` _returnvalue_z (+ _returnvalue_z 100.0) _runtrack)) false false))
      (:`Finished`
        (`self.K2_DestroyActor`)))))

(event `self.Box.OnComponentBeginOverlap`
  (params (OverlappedComponent :type "PrimitiveComponent Object Reference") (OtherActor :type "Actor Object Reference") (OtherComp :type "PrimitiveComponent Object Reference") (OtherBodyIndex :type Integer) (bFromSweep :type Boolean) (SweepResult :type "HitResult Structure (by ref)"))
  (bind _asside_scroller_character (cast `/Game/SideScrollerBP/Blueprints/SideScrollerCharacter` OtherActor))
  (`/Game/SideScrollerBP/Blueprints/SideScrollerCharacter.Death` _asside_scroller_character))

(fn `UserConstructionScript`)