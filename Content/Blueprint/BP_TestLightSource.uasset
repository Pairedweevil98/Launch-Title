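; BP_TestLightSource is a test light-source actor that rotates in steps when interacted with while the SideScrollerCharacter is inside its box.
; Box overlaps gate the Interact event, which plays one of two timelines that add an offset to the root's stored roll.
; DoOnce nodes block retriggering until each timeline finishes and saves the new rotation.
; A turn counter flips AddOrSub after several turns, alternating between the two timelines.
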(event `/Game/Blueprint/BPI_Interact.Interact`
  (if (`self.PlayerInBox?`)
    (if (`self.AddOrSub`)
      (`/Engine/EditorBlueprintResources/StandardMacros.DoOnce` false :!label _label
        (:`Completed`
          (bind (_direction _rotatetrack) (`Timeline|RotateTimeline` :!via `PlayFromStart`)
            (:`Update`
              (bind _returnvalue (+ _rotatetrack (`self.CurrentRotation`)))
              (`SceneComponent.K2_SetWorldRotation` (`self.DefaultSceneRoot`) (`KismetMathLibrary.MakeRotator` _returnvalue) false false))
            (:`Finished`
              (set `self.CurrentRotation` _returnvalue)
              (`|ExecutionSequence`
                (:`then_0`
                  (bind _result (`/Engine/EditorBlueprintResources/StandardMacros.IncrementInt` (`self.CurrentTurn`))
                    (:`  `
                      (if (> _result 3)
                        (set `self.AddOrSub` false)
                        (set `self.CurrentTurn` 0)))))
                (:`then_1`
                  (goto _label :!via `Reset`)))))))
      (else
        (`/Engine/EditorBlueprintResources/StandardMacros.DoOnce` false :!label _label_2
          (:`Completed`
            (bind (_direction_2 _rotatetrack_2) (`Timeline|Timeline_0` :!via `PlayFromStart`)
              (:`Update`
                (bind _returnvalue_2 (+ _rotatetrack_2 (`self.CurrentRotation`)))
                (`SceneComponent.K2_SetWorldRotation` (`self.DefaultSceneRoot`) (`KismetMathLibrary.MakeRotator` _returnvalue_2) false false))
              (:`Finished`
                (set `self.CurrentRotation` _returnvalue_2)
                (`|ExecutionSequence`
                  (:`then_0`
                    (bind _result_2 (`/Engine/EditorBlueprintResources/StandardMacros.IncrementInt` (`self.CurrentTurn`))
                      (:`  `
                        (if (> _result_2 3)
                          (set `self.AddOrSub` true)
                          (set `self.CurrentTurn` 0)))))
                  (:`then_1`
                    (goto _label_2 :!via `Reset`)))))))))))

(event `self.Box.OnComponentBeginOverlap`
  (params (OverlappedComponent :type "PrimitiveComponent Object Reference") (OtherActor :type "Actor Object Reference") (OtherComp :type "PrimitiveComponent Object Reference") (OtherBodyIndex :type Integer) (bFromSweep :type Boolean) (SweepResult :type "HitResult Structure (by ref)"))
  (cast `/Game/SideScrollerBP/Blueprints/SideScrollerCharacter` OtherActor)
  (set `self.PlayerInBox?` true))

(event `self.Box.OnComponentEndOverlap`
  (params (OverlappedComponent :type "PrimitiveComponent Object Reference") (OtherActor :type "Actor Object Reference") (OtherComp :type "PrimitiveComponent Object Reference") (OtherBodyIndex :type Integer))
  (cast `/Game/SideScrollerBP/Blueprints/SideScrollerCharacter` OtherActor)
  (set `self.PlayerInBox?` false))

(fn `UserConstructionScript`)