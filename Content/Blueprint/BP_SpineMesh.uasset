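; Spline actor that builds a continuous run of mesh sections, apparently rails, along its spline in the construction script.
; It adds one spline mesh component per whole section length, with tangents clamped to that length for even bending.
; Section length is actor X scale times a coefficient that the loop refreshes from mesh X bounds only after the length is computed.
; The event graph has no active logic.
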(fn `UserConstructionScript`
  (bind _returnvalue_x (`KismetMathLibrary.BreakVector` (`self.GetActorScale3D`)))
  (bind _sectionlength (`self.SectionLength`))
  (bind _sectionlength_2 (`self.SectionLength`))
  (bind _returnvalue (* (`self.CurrentIndex`) (`self.SectionLength`)))
  (bind _returnvalue_2 (* (+ (`self.CurrentIndex`) 1) (`self.SectionLength`)))
  (bind (_min _max) (break `Box` (`StaticMesh.GetBoundingBox` (`StaticMeshComponent.StaticMesh` (`self.RailsSpline`)))))
  (set `self.SectionLength` (* _returnvalue_x (`self.SectionLengthCoef`)))
  (for _index (range (`KismetMathLibrary.FTrunc` (/ (`SplineComponent.GetSplineLength` (`self.Spline`)) (`self.SectionLength`))))
    (set `self.CurrentIndex` _index)
    (bind _returnvalue_3 (`AddComponent|NODE_AddSplineMeshComponent-1`))
    (set `self.RailsSpline` _returnvalue_3)
    (set `self.SectionLengthCoef` (- (.x _max) (.x _min)))
    (`SplineMeshComponent.SetStartAndEnd` (`self.RailsSpline`) (`SplineComponent.GetLocationAtDistanceAlongSpline` (`self.Spline`) _returnvalue "Local") (`KismetMathLibrary.ClampVectorSize` (`SplineComponent.GetTangentAtDistanceAlongSpline` (`self.Spline`) _returnvalue "Local") _sectionlength_2 _sectionlength_2) (`SplineComponent.GetLocationAtDistanceAlongSpline` (`self.Spline`) _returnvalue_2 "Local") (`KismetMathLibrary.ClampVectorSize` (`SplineComponent.GetTangentAtDistanceAlongSpline` (`self.Spline`) _returnvalue_2 "Local") _sectionlength _sectionlength) true)))