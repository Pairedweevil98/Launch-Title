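; BP_ControlsPopUp is a trigger actor that pops up a plane, likely showing controls, when the player character is nearby.
; The plane starts at zero scale, and entering the box plays the ScaleTL timeline to grow it in X and Y.
; Leaving the box reverses the timeline to shrink it, with DoOnce gates guarding against repeated triggers.
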(event `self.ReceiveBeginPlay`
  (`SceneComponent.SetWorldScale3D` (`self.Plane`) (0.0 0.0 0.0)))

(event `self.Box.OnComponentBeginOverlap`
  (params (OverlappedComponent :type "PrimitiveComponent Object Reference") (OtherActor :type "Actor Object Reference") (OtherComp :type "PrimitiveComponent Object Reference") (OtherBodyIndex :type Integer) (bFromSweep :type Boolean) (SweepResult :type "HitResult Structure (by ref)"))
  (if (== OtherActor (`GameplayStatics.GetPlayerCharacter` 0))
    (`/Engine/EditorBlueprintResources/StandardMacros.DoOnce` false
      (:`Completed`
        (`|ExecutionSequence`
          (:`then_0`
            (bind (_direction _alpha) (`Timeline|ScaleTL` :!label _label)
              (:`Update`
                (bind _returnvalue (`KismetMathLibrary.Lerp` 0.0 1.5 _alpha))
                (`SceneComponent.SetWorldScale3D` (`self.Plane`) (`KismetMathLibrary.MakeVector` _returnvalue _returnvalue 1.0)))))
          (:`then_1`
            (goto _label_2 :!via `Reset`)))))))

(event `self.Box.OnComponentEndOverlap`
  (params (OverlappedComponent :type "PrimitiveComponent Object Reference") (OtherActor :type "Actor Object Reference") (OtherComp :type "PrimitiveComponent Object Reference") (OtherBodyIndex :type Integer))
  (if (== OtherActor (`GameplayStatics.GetPlayerCharacter` 0))
    (`/Engine/EditorBlueprintResources/StandardMacros.DoOnce` false :!label _label_2
      (:`Completed`
        (`|ExecutionSequence`
          (:`then_0`
            (goto _label :!via `Reverse`)))))))

(fn `UserConstructionScript`)