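; BP_DashCrystal is a dash pickup that temporarily enables DashActive on an overlapping SideScrollerCharacter.
; A DoOnce-gated Box overlap hides the Cube, disables its collision, turns on green character particles and starts a timeline.
; The timeline's event track drives a FlipFlop that toggles Cube visibility.
; When the timeline finishes, it clears DashActive, updates the particles and resets the DoOnce, leaving Cube collision off.
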(event `self.Box.OnComponentBeginOverlap`
  (params (OverlappedComponent :type "PrimitiveComponent Object Reference") (OtherActor :type "Actor Object Reference") (OtherComp :type "PrimitiveComponent Object Reference") (OtherBodyIndex :type Integer) (bFromSweep :type Boolean) (SweepResult :type "HitResult Structure (by ref)"))
  (bind _cube (`self.Cube`))
  (bind _cube_2 (`self.Cube`))
  (bind _asside_scroller_character (cast `/Game/SideScrollerBP/Blueprints/SideScrollerCharacter` OtherActor))
  (`/Engine/EditorBlueprintResources/StandardMacros.DoOnce` false :!label _label
    (:`Completed`
      (bind _output_get (set `/Game/SideScrollerBP/Blueprints/SideScrollerCharacter.DashActive` true _asside_scroller_character))
      (`SceneComponent.SetVisibility` _cube false false)
      (`PrimitiveComponent.SetCollisionEnabled` _cube "NoCollision")
      (`/Game/SideScrollerBP/Blueprints/SideScrollerCharacter.SetParticles` _asside_scroller_character (struct :`G` 1.0 :`A` 1.0) _output_get)
      (`Timeline|Timeline_0` :!via `PlayFromStart`
        (:`Finished`
          (bind _output_get_2 (set `/Game/SideScrollerBP/Blueprints/SideScrollerCharacter.DashActive` false _asside_scroller_character))
          (`self.Reset`)
          (`/Game/SideScrollerBP/Blueprints/SideScrollerCharacter.SetParticles` _asside_scroller_character (struct :`G` 1.0 :`A` 1.0) _output_get_2))
        (:`VisiblityTrack`
          (`/Engine/EditorBlueprintResources/StandardMacros.FlipFlop`
            (:`A`
              (`SceneComponent.SetVisibility` _cube_2 true false))
            (:`B`
              (`SceneComponent.SetVisibility` _cube_2 false false))))))))

(event `Reset`
  (goto _label :!via `Reset`))

(fn `UserConstructionScript`)