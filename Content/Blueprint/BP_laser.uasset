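; Laser emitter for a side-scroller that the player, while inside its Box, switches on with Interact and rotates on later interactions.
; Two timelines turn the mesh in steps, reversing direction after a set number of turns and recasting the light every update.
; LightRay rebuilds the BP_LaserBeam segments by repeated line traces, reflecting off surfaces identified by material and making any Spider it hits run away.
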(event `/Game/Blueprint/BPI_Interact.Interact`
  (bind _staticmesh (`self.StaticMesh`))
  (if (`self.PlayerInBox?`)
    (if (`self.LightOn?`)
      (if (`self.AddOrSub`)
        (`/Engine/EditorBlueprintResources/StandardMacros.DoOnce` false :!label _label
          (:`Completed`
            (bind (_direction _rotatetrack) (`Timeline|Timeline_0` :!via `PlayFromStart`)
              (:`Update`
                (bind _returnvalue (+ _rotatetrack (`self.CurrentRotation`)))
                (`SceneComponent.K2_SetWorldRotation` _staticmesh (`KismetMathLibrary.MakeRotator` _returnvalue) false false)
                (`self.CastLight`))
              (:`Finished`
                (set `self.CurrentRotation` _returnvalue)
                (`|ExecutionSequence`
                  (:`then_0`
                    (bind _result (`/Engine/EditorBlueprintResources/StandardMacros.IncrementInt` (`self.CurrentTurn`))
                      (:`  `
                        (if (> _result 3)
                          (set `self.AddOrSub` false)
                          (set `self.CurrentTurn` 0)))))
                  (:`then_1`
                    (goto _label :!via `Reset`)))))))
        (else
          (`/Engine/EditorBlueprintResources/StandardMacros.DoOnce` false :!label _label_2
            (:`Completed`
              (bind (_direction_2 _rotatetrack_2) (`Timeline|Timeline_1` :!via `PlayFromStart`)
                (:`Update`
                  (bind _returnvalue_2 (+ _rotatetrack_2 (`self.CurrentRotation`)))
                  (`SceneComponent.K2_SetWorldRotation` _staticmesh (`KismetMathLibrary.MakeRotator` _returnvalue_2) false false)
                  (`self.CastLight`))
                (:`Finished`
                  (set `self.CurrentRotation` _returnvalue_2)
                  (`|ExecutionSequence`
                    (:`then_0`
                      (bind _result_2 (`/Engine/EditorBlueprintResources/StandardMacros.IncrementInt` (`self.CurrentTurn`))
                        (:`  `
                          (if (> _result_2 3)
                            (set `self.AddOrSub` true)
                            (set `self.CurrentTurn` 0)))))
                    (:`then_1`
                      (goto _label_2 :!via `Reset`)))))))))
      (else
        (`self.CastLight`)))))

(event `self.Box.OnComponentBeginOverlap`
  (params (OverlappedComponent :type "PrimitiveComponent Object Reference") (OtherActor :type "Actor Object Reference") (OtherComp :type "PrimitiveComponent Object Reference") (OtherBodyIndex :type Integer) (bFromSweep :type Boolean) (SweepResult :type "HitResult Structure (by ref)"))
  (cast `/Game/SideScrollerBP/Blueprints/SideScrollerCharacter` OtherActor)
  (set `self.PlayerInBox?` true))

(event `self.Box.OnComponentEndOverlap`
  (params (OverlappedComponent :type "PrimitiveComponent Object Reference") (OtherActor :type "Actor Object Reference") (OtherComp :type "PrimitiveComponent Object Reference") (OtherBodyIndex :type Integer))
  (cast `/Game/SideScrollerBP/Blueprints/SideScrollerCharacter` OtherActor)
  (set `self.PlayerInBox?` false))

(event `CastLight`
  (bind _arrow (`self.Arrow`))
  (set `self.LightOn?` true)
  (`self.LightRay` (`SceneComponent.K2_GetComponentLocation` _arrow) (`SceneComponent.GetForwardVector` _arrow) (`self.Distance`)))

(fn `LightRay`
  (params (OriginLoc :type "Vector Structure") (Direction :type "Vector Structure") (Distance :type "Float (double-precision)"))
  (locals (L_OriginLoc :type "Vector Structure") (L_Direction :type "Vector Structure") (L_Distance :type "Float (double-precision)") (L_Continue :type Boolean :default true) (L_StartBeamLoc :type "Vector Structure") (L_EndBeamLoc :type "Vector Structure"))
  (bind _l_originloc (`local.L_OriginLoc`))
  (bind _beams (`self.Beams`))
  (set `local.L_OriginLoc` OriginLoc)
  (set `local.L_Direction` Direction)
  (set `local.L_Distance` Distance)
  (for _array_element _beams
    (`self.K2_DestroyActor` _array_element))
  (`KismetArrayLibrary.Array_Clear` _beams)
  (while (`local.L_Continue`)
    (`|ExecutionSequence`
      (:`then_0`
        (bind (_outhit _returnvalue) (`KismetSystemLibrary.LineTraceSingle` _l_originloc (+ _l_originloc (* (`local.L_Direction`) (`local.L_Distance`))) "TraceTypeQuery3" true))
        (set `local.L_StartBeamLoc` (`local.L_OriginLoc`))
        (if _returnvalue
          (bind (_bblockinghit _binitialoverlap _time _distance _location _impactpoint _normal _impactnormal _physmat _hitactor _hitcomponent _hitbonename _hititem _faceindex _tracestart _traceend) (`GameplayStatics.BreakHitResult` _outhit))
          (set `local.L_EndBeamLoc` _impactpoint)
          (bind (_sectionindex _returnvalue_2) (`PrimitiveComponent.GetMaterialFromCollisionFaceIndex` _hitcomponent _faceindex))
          (if (== _returnvalue_2 "/Engine/BasicShapes/BasicShapeMaterial.BasicShapeMaterial")
            (set `local.L_OriginLoc` _impactpoint)
            (set `local.L_Direction` (`KismetMathLibrary.MirrorVectorByNormal` (`local.L_Direction`) _impactnormal))
            (set `local.L_Continue` true)
            (else
              (if (== _returnvalue_2 "/Game/Materials/MI_Spider.MI_Spider")
                (bind _asspider (cast `/Game/Blueprint/Spider` _hitactor))
                (`/Game/Blueprint/Spider.RunAway` _asspider))
              (set `local.L_Continue` false :!label _label)))
          (else
            (set `local.L_EndBeamLoc` _traceend)
            (goto _label))))
      (:`then_1`
        (bind _returnvalue_3 (`|SpawnActorFromClass` "/Game/Blueprint/BP_LaserBeam.BP_LaserBeam_C" (`KismetMathLibrary.MakeTransform` (0.0 0.0 0.0)) "Undefined" "OverrideRootScale" null null))
        (`/Game/Blueprint/BP_LaserBeam.Set End` _returnvalue_3 (`local.L_StartBeamLoc`) (`local.L_EndBeamLoc`))
        (`KismetArrayLibrary.Array_Add` (`self.Beams`) _returnvalue_3)))))

(fn `UserConstructionScript`)