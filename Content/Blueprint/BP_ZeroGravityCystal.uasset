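; A single-use zero-gravity crystal pickup that temporarily lowers the side-scroller character's gravity.
; A box overlap fires once, lowers GravityScale, turns on purple particles on the character, and hides the cube and disables its collision.
; A timeline times the effect, its event track flip-flopping cube visibility.
; When it finishes, gravity is set to a fixed 2.0 and the particles switch off.
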(event `self.Box.OnComponentBeginOverlap`
  (params (OverlappedComponent :type "PrimitiveComponent Object Reference") (OtherActor :type "Actor Object Reference") (OtherComp :type "PrimitiveComponent Object Reference") (OtherBodyIndex :type Integer) (bFromSweep :type Boolean) (SweepResult :type "HitResult Structure (by ref)"))
  (bind _cube (`self.Cube`))
  (bind _cube_2 (`self.Cube`))
  (bind _asside_scroller_character (cast `/Game/SideScrollerBP/Blueprints/SideScrollerCharacter` OtherActor))
  (`/Engine/EditorBlueprintResources/StandardMacros.DoOnce` false
    (:`Completed`
      (bind _output_get (set `self.Active` true))
      (`/Game/SideScrollerBP/Blueprints/SideScrollerCharacter.SetParticles` _asside_scroller_character (struct :`R` 0.504 :`B` 1.0 :`A` 1.0) _output_get)
      (bind _charactermovement (`Character.CharacterMovement` _asside_scroller_character))
      (set `CharacterMovementComponent.GravityScale` 0.5 _charactermovement)
      (`SceneComponent.SetVisibility` _cube_2 false false)
      (`PrimitiveComponent.SetCollisionEnabled` _cube_2 "NoCollision")
      (`Timeline|Timeline_0` :!via `PlayFromStart`
        (:`Finished`
          (set `CharacterMovementComponent.GravityScale` 2.0 _charactermovement)
          (bind _output_get_2 (set `self.Active` false))
          (`/Game/SideScrollerBP/Blueprints/SideScrollerCharacter.SetParticles` :`self` _asside_scroller_character :`ToggleOnOff` _output_get_2))
        (:`VisiblityTrack`
          (`/Engine/EditorBlueprintResources/StandardMacros.FlipFlop`
            (:`A`
              (`SceneComponent.SetVisibility` _cube true false))
            (:`B`
              (`SceneComponent.SetVisibility` _cube false false))))))))

(fn `UserConstructionScript`)