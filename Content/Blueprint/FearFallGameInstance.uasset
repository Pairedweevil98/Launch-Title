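; FearFallGameInstance holds the unlock flags for levels 2 and 3 and persists them to a save slot.
; Save loads the existing "save1" FearFallSaveGame, copies the flags into it and writes it back, doing nothing if the cast fails.
; Load reads the flags back from that slot.
; The save object's fields are named Locked but store the Unlocked values directly, without inversion.
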(fn `Load`
  (bind _returnvalue (`GameplayStatics.LoadGameFromSlot` "save1"))
  (bind _asfear_fall_save_game (cast `/Game/Blueprint/FearFallSaveGame` _returnvalue))
  (set `self.Level2Unlocked` (`/Game/Blueprint/FearFallSaveGame.SGLevel2Locked` _asfear_fall_save_game))
  (set `self.Level3Unlocked` (`/Game/Blueprint/FearFallSaveGame.SGLevel3Locked` _asfear_fall_save_game)))

(fn `Save`
  (bind _returnvalue (`GameplayStatics.LoadGameFromSlot` "save1"))
  (bind _asfear_fall_save_game (cast `/Game/Blueprint/FearFallSaveGame` _returnvalue))
  (set `/Game/Blueprint/FearFallSaveGame.SGLevel2Locked` (`self.Level2Unlocked`) _asfear_fall_save_game)
  (set `/Game/Blueprint/FearFallSaveGame.SGLevel3Locked` (`self.Level3Unlocked`) _asfear_fall_save_game)
  (`GameplayStatics.SaveGameToSlot` _asfear_fall_save_game "save1"))