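; BP_PlaySequencer is a trigger actor that plays a level sequence once when the player character overlaps its box.
; With ChangeCamera set, it blends the view to its camera and disables input during playback.
; A delay based on the sequence's end time precedes re-enabling input and, in camera mode, blending back to the player.
; The construction script locks the actor's world X to a fixed value, keeping Y and Z.
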(event `self.Box.OnComponentBeginOverlap`
  (params (OverlappedComponent :type "PrimitiveComponent Object Reference") (OtherActor :type "Actor Object Reference") (OtherComp :type "PrimitiveComponent Object Reference") (OtherBodyIndex :type Integer) (bFromSweep :type Boolean) (SweepResult :type "HitResult Structure (by ref)"))
  (bind _sequenceplayer (`LevelSequenceActor.SequencePlayer` (`self.Sequence`)))
  (bind _sequenceplayer_2 (`LevelSequenceActor.SequencePlayer` (`self.Sequence`)))
  (if (== OtherActor (`GameplayStatics.GetPlayerCharacter` 0))
    (`/Engine/EditorBlueprintResources/StandardMacros.DoOnce` false
      (:`Completed`
        (if (`self.ChangeCamera?`)
          (`PlayerController.SetViewTargetWithBlend` (`GameplayStatics.GetPlayerController` 0) (`self.Camera`) (`self.BlendTime`) "VTBlend_Linear" 0.0 false)
          (`self.DisableInput` (`GameplayStatics.GetPlayerCharacter` 0) (`GameplayStatics.GetPlayerController` 0))
          (`MovieSceneSequencePlayer.Play` _sequenceplayer_2)
          (`KismetSystemLibrary.Delay` (+ (`TimeManagementBlueprintLibrary.Conv_QualifiedFrameTimeToSeconds` (`MovieSceneSequencePlayer.GetEndTime` _sequenceplayer_2)) 0.1))
          (`PlayerController.SetViewTargetWithBlend` (`GameplayStatics.GetPlayerController` 0) (`GameplayStatics.GetPlayerCharacter` 0) (`self.BlendTime`) "VTBlend_Linear" 0.0 false)
          (`self.EnableInput` (`GameplayStatics.GetPlayerCharacter` 0) (`GameplayStatics.GetPlayerController` 0))
          (else
            (`MovieSceneSequencePlayer.Play` _sequenceplayer)
            (`KismetSystemLibrary.Delay` (+ (`TimeManagementBlueprintLibrary.Conv_QualifiedFrameTimeToSeconds` (`MovieSceneSequencePlayer.GetEndTime` _sequenceplayer)) 0.1))
            (`self.EnableInput` (`GameplayStatics.GetPlayerCharacter` 0) (`GameplayStatics.GetPlayerController` 0))))))))

(fn `UserConstructionScript`
  (bind (_returnvalue_x _returnvalue_y _returnvalue_z) (`KismetMathLibrary.BreakVector` (`self.K2_GetActorLocation`)))
  (`self.K2_SetActorLocation` (`KismetMathLibrary.MakeVector` 1200.0 _returnvalue_y _returnvalue_z)))